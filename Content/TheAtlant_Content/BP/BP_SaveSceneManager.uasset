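; BP_SaveSceneManager is a scene save manager that builds a list of save data for a level's objects.
; On BeginPlay it copies the object list for its ID from the GI_TheAtlant game instance.
; If that list is not empty, it appends an entry per CurrentObject actor, holding display name, transform and a false IsAlive flag.
; The updated list is not written back to the game instance here.
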(event `self.ReceiveBeginPlay`
  ;[1 1 1] Get Object list
  (bind _asgi_the_atlant (cast `/Game/TheAtlant_Content/BP/Game/GI_TheAtlant` (`GameplayStatics.GetGameInstance`)))
  (bind _output_get (set `self.SaveObjectList` (`.ObjectList_3_5B121CE8438B2E4E9ECD64A1D55D76AC` (break `/Game/TheAtlant_Content/Data/Struct/S_SaveLevelData` (`|GetArrayItem` (`/Game/TheAtlant_Content/BP/Game/GI_TheAtlant.SaveLevelList` _asgi_the_atlant) (`self.ID`))))))
  ;[1 1 1] Look if has created object list
  (if (not (== (`KismetArrayLibrary.Array_Length` _output_get) 0))
    ;[1 1 1] Create list
    (for _array_element (`self.CurrentObject`)
      (`self.CreateNewSaveObjectDataEntry` _array_element))))

(fn `CreateNewSaveObjectDataEntry`
  (params (Actor :type "Actor Object Reference"))
  (`KismetArrayLibrary.Array_Add` (`self.SaveObjectList`) (make `/Game/TheAtlant_Content/Data/Struct/S_SaveObjectData` (`KismetSystemLibrary.GetDisplayName` Actor) (`self.GetTransform` Actor))))

(fn `UserConstructionScript`)