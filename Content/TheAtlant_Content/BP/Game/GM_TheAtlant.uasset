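; GM_TheAtlant is the game mode that respawns the player after the character is destroyed.
; On BeginPlay it binds to the BP_Player's OnDestroyed event.
; After a delay it spawns a new BP_Player at the game instance's respawn transform, possesses it, restores the gameplay input mapping and rebinds.
; It then stores the new pawn on PC_TheAtlant and broadcasts it through an event dispatcher, marked as temporary.
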(event `Respawn`
  (bind _asbp_player (cast `/Game/TheAtlant_Content/BP/BP_Player` (`GameplayStatics.GetPlayerCharacter` 0) :!label _label))
  (add `self.OnDestroyed` _asbp_player (delegate `OnPlayerDestroyed`)))

(event `self.ReceiveBeginPlay`
  (goto _label))

(event `OnPlayerDestroyed` :!signature `self.OnDestroyed`
  (params (DestroyedActor :type "Actor Object Reference"))
  (bind _returnvalue (`GameplayStatics.GetPlayerController` 0))
  (`KismetSystemLibrary.Delay` (`self.RespawnTime`))
  ;[1 1 1] Player respawn
  (bind _asgi_the_atlant (cast `/Game/TheAtlant_Content/BP/Game/GI_TheAtlant` (`GameplayStatics.GetGameInstance`)))
  (bind _returnvalue_2 (`|SpawnActorFromClass` "/Game/TheAtlant_Content/BP/BP_Player.BP_Player_C" (`/Game/TheAtlant_Content/BP/Game/GI_TheAtlant.PlayerRespawnTransform` _asgi_the_atlant) "Undefined" "MultiplyWithRoot" null null))
  (`KismetSystemLibrary.PrintString` (`KismetStringLibrary.Concat_StrStr` "BP_Player:" (`KismetSystemLibrary.GetObjectName` _returnvalue_2) "Player controller: " (`KismetSystemLibrary.GetObjectName` _returnvalue)))
  (`Controller.Possess` _returnvalue _returnvalue_2)
  (message `EnhancedInputSubsystemInterface.AddMappingContext` (pcsubsystem `EnhancedInputLocalPlayerSubsystem` _returnvalue) "/Game/TheAtlant_Content/Input/IMC_Gameplay.IMC_Gameplay" 0 (struct))
  (`self.Respawn`)
  ;;[1 1 1] Temp, need to make an event that everything that needs the player reference subscribes to it
  (bind _aspc_the_atlant (cast `/Game/TheAtlant_Content/BP/Game/PC_TheAtlant` (`GameplayStatics.GetPlayerController` 0)))
  (bind _output_get (set `/Game/TheAtlant_Content/BP/Game/PC_TheAtlant.BP_Player` _returnvalue_2 _aspc_the_atlant))
  (`/Game/TheAtlant_Content/BP/Game/PC_TheAtlant.ED_OnGotNewPlayer` _aspc_the_atlant _output_get))

(fn `UserConstructionScript`)