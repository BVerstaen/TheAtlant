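; Jellyfish enemy that leaps onto an overlapping player's face and damages them on a looping timer while a quick-time event runs.
; A timeline lerps it to the player's jump point, where it attaches and launches the QTE through the player's event dispatcher.
; CE_StopQTE counts down remaining hits, then explodes and kills the jelly, redrawing the harpoon unless player death sent the -666 sentinel.
; MetaSound triggers drive randomly timed idle and attack audio.
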(event `self.ReceiveBeginPlay`
  ;[1 1 1] Get default
  (set `self.DefaultTransform` (`self.GetTransform`))
  ;[1 1 1] Guard
  (if (> (`self.NumberOfHit`) 0)
    (if (> (`self.TimeBTWAttack`) 0.0)
      (if (not (> (`self.Damage`) 0))
        (`KismetSystemLibrary.PrintString` "Damage can't be negative" false))
      (else
        (`KismetSystemLibrary.PrintString` "TimeBTWAttack can't be negative" false)))
    (else
      (`KismetSystemLibrary.PrintString` "Number of hit can't be negative" false))))

(event `self.ReceiveActorBeginOverlap`
  (params (OtherActor :type "Actor Object Reference"))
  ;[1 1 1] If is in range of player
  (if (not (`self.IsDying`))
    (bind _asbp_player (cast `/Game/TheAtlant_Content/BP/BP_Player` OtherActor))
    (`self.CE_AttackPlayer` _asbp_player)))

(event `CE_AttackPlayer`
  (params (Player :type "/Game/TheAtlant_Content/BP/BP_Player Object Reference"))
  ;[1 1 1] Get player & check if not
  (bind _output_get (set `self.PlayerActor` Player))
  (`/Game/TheAtlant_Content/BP/BP_Player.CE_PlayHarpoonHide` _output_get)
  (add `/Game/TheAtlant_Content/BP/BP_Player.ED_OnPlayerDied` _output_get (delegate `CE_DeathKill`))
  ;[1 1 1] Jump into player face
  (bind (_direction _jumplerp) (`Timeline|tl_JumpToPlayer`)
    (:`Update`
      (bind _playeractor (`self.PlayerActor`)
        (:`then`
          (bind _jellyjumppoint (`/Game/TheAtlant_Content/BP/BP_Player.JellyJumpPoint` _playeractor)
            (:`then`
              (`self.K2_SetActorTransform` (`KismetMathLibrary.TLerp` (`self.DefaultTransform`) (`SceneComponent.K2_GetComponentToWorld` _jellyjumppoint) _jumplerp)))
            (:`else`)))
        (:`else`)))
    (:`Finished`
      (`self.StopIdleSounds`)
      (if (not (`self.IsAttacking`))
        (set `self.IsAttacking` true)
        ;[1 0.3326 0.9534] Sound
        (bind _returnvalue (`GameplayStatics.SpawnSoundAtLocation` "/Game/TheAtlant_Content/Audio/_MetaSounds/Jellyfish/MS_Jellyfish.MS_Jellyfish" (`SceneComponent.K2_GetComponentLocation` (`self.Collision`)) (struct) 1.0 1.0 0.0 null null))
        (`AudioParameterControllerInterface.SetTriggerParameter` _returnvalue "Attack"))
      ;[1 1 1] Attach to scene component
      (bind _playeractor_2 (`self.PlayerActor`)
        (:`then`
          (bind _jellyjumppoint_2 (`/Game/TheAtlant_Content/BP/BP_Player.JellyJumpPoint` _playeractor_2)
            (:`then`
              (`self.K2_AttachToComponent` _jellyjumppoint_2 "None" "KeepWorld" "KeepWorld" "KeepWorld")
              ;[1 1 1] Activate QTE
              (`/Game/TheAtlant_Content/BP/BP_Player.ED_OnLaunchQTE` _playeractor_2 (`self.NumberOfHit`))
              (add `/Game/TheAtlant_Content/BP/BP_Player.ED_OnLaunchQTE` _playeractor_2 (`|CreateDelegate` :!event `CE_StopQTE`))
              ;[1 1 1] Timer to attack player
              (`KismetSystemLibrary.K2_SetTimerDelegate` (delegate `CE_DamagePlayer`) (`self.TimeBTWAttack`) true))
            (:`else`)))
        (:`else`)))))

(event `CE_DeathKill`
  ;[1 1 1] Kill Jelly if player died (-666 = doesn't draw harpoon)
  (`self.CE_StopQTE` -666))

(event `CE_StopQTE`
  (params (Hit :type Integer))
  ;[1 1 1] Damage & kill jelly
  (if (not (> Hit 0))
    (`/Engine/EditorBlueprintResources/StandardMacros.DecrementInt` (`self.NumberOfHit`)
      (:`  `
        (if (not (> (`self.NumberOfHit`) 0))
          (`GameplayStatics.SpawnEmitterAtLocation` "/Game/StarterContent/Particles/P_Explosion.P_Explosion" (`self.K2_GetActorLocation`) (`self.K2_GetActorRotation`))
          ;;[1 1 1] Draw harpoon if needed
          (if (not (== Hit -666))
            (bind _playeractor (`self.PlayerActor`)
              (:`then`
                (`/Game/TheAtlant_Content/BP/BP_Player.CE_PlayHarpoonDraw` _playeractor))
              (:`else`)))
          (`self.JellyStopAttackound`)
          (set `self.IsDying` true)
          (bind _skeletalmesh (`self.SkeletalMesh`)
            (:`then`
              (`SkeletalMeshComponent.PlayAnimation` _skeletalmesh "/Game/TheAtlant_Content/GA/Jellyfish/Jellyfish/Anim/kill_anim_jellyfish.kill_anim_jellyfish" false)
              (`KismetSystemLibrary.Delay` 1.8)
              (`self.K2_DestroyActor`))
            (:`else`)))))))

(event `JellyStopAttackound`
  ;[1 0.4475 0.8689] StopSound
  (if (`KismetSystemLibrary.IsValid` (stale `CE_AttackPlayer` _returnvalue))
    (`AudioComponent.FadeOut` (stale `CE_AttackPlayer` _returnvalue) 1.0 0.0 "Linear")))

(event `self.ReceiveTick`
  (params (DeltaSeconds :type "Float (single-precision)"))
  ;[0.3047 1 0.6059] Idle Sounds
  (if (`self.IsAttacking`)
    _
    (elif (not (`self.IsAwaitingIdle`))
      (`KismetSystemLibrary.K2_SetTimerDelegate` (delegate `TimerDone`) (`KismetMathLibrary.RandomFloatInRange` (`self.MinAudioDelay`) (`self.MaxAudioDelay`)))
      (set `self.IsAwaitingIdle` true))))

(event `StopIdleSounds`
  ;[0.6204 1 0.4004] StopIdleSounds
  (if (`KismetSystemLibrary.IsValid` (stale `TimerDone` _returnvalue))
    (`AudioComponent.FadeOut` (stale `TimerDone` _returnvalue) 0.3 0.0 "Linear")))

(event `CE_DamagePlayer`
  ;[1 1 1] Timer to attack player
  ;;[1 1 1] Attack player
  (bind _playeractor (`self.PlayerActor`)
    (:`then`
      (`/Game/TheAtlant_Content/BP/BP_Player.CE_PlayerHit` _playeractor 2))
    (:`else`)))

(event `TimerDone`
  ;[0.3047 1 0.6059] Idle Sounds
  (set `self.IsAwaitingIdle` false)
  (bind _returnvalue (`GameplayStatics.SpawnSoundAtLocation` "/Game/TheAtlant_Content/Audio/_MetaSounds/Jellyfish/MS_Jellyfish.MS_Jellyfish" (`SceneComponent.K2_GetComponentLocation` (`self.Collision`)) (struct) 1.0 1.0 0.0 null null))
  (`AudioParameterControllerInterface.SetTriggerParameter` _returnvalue "Idle"))

(fn `UserConstructionScript`)