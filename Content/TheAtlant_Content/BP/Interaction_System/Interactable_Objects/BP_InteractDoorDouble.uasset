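; Interactable double door that swings both leaves open or closed with a timeline-driven yaw lerp and open/close sounds.
; Direct interaction toggles it, or plays a locked sound if it needs a lever or key.
; Linked levers decrement a required count and toggle the door once it reaches zero or below.
; GetID exposes the door's Id, and debug strings print on toggle and lever pulls.
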(event `ToggleDoor`
  ;[1 0.4992 0.6615] Door animation
  (if (`self._isClosed`)
    (`GameplayStatics.PlaySoundAtLocation` (`self.DoorSoundOpen`) (`SceneComponent.K2_GetComponentLocation` (`self.Door`)) (struct) 1.0 1.0 0.0 null null null null)
    (set `self._isClosed` false)
    (`KismetSystemLibrary.PrintString` "OPEN" false)
    (bind (_direction _alpha) (`Timeline|TM_Door` :!label _label)
      (:`Update`
        (`SceneComponent.K2_SetRelativeRotation` (`self.Door`) (`KismetMathLibrary.MakeRotator` 0.0 0.0 (`KismetMathLibrary.Lerp` 0.0 90.0 _alpha)) false false)
        (`SceneComponent.K2_SetRelativeRotation` (`self.Door1`) (`KismetMathLibrary.MakeRotator` 0.0 0.0 (`KismetMathLibrary.Lerp` 180.0 90.0 _alpha)) false false)))
    (else
      (`GameplayStatics.PlaySoundAtLocation` (`self.DoorSoundClose`) (`SceneComponent.K2_GetComponentLocation` (`self.Door`)) (struct) 1.0 1.0 0.0 null null null null)
      (set `self._isClosed` true)
      (`KismetSystemLibrary.PrintString` "CLOSE" false)
      (goto _label :!via `Reverse`))))

(event `LeverPulled`
  ;[1 0.8153 0.3173] A lever linked to this door has been pulled
  (`KismetSystemLibrary.PrintString` "I am door" false)
  (bind _result (`/Engine/EditorBlueprintResources/StandardMacros.DecrementInt` (`self._numLeversNeeded`))
    (:`  `
      (bind _output_get (set `self._numLeversNeeded` _result))
      (if (<= _output_get 0)
        (`self.ToggleDoor`)))))

(event `self.Interact`
  ;[1 1 1] Regular interact
  (if (`self._needsLever`)
    (`GameplayStatics.PlaySoundAtLocation` "/Game/TheAtlant_Content/Audio/LockedDoor1.LockedDoor1" (`SceneComponent.K2_GetComponentLocation` (`self.Door`)) (struct) 1.0 1.0 0.0 null null null null :!label _label_2)
    (elif (`self._needsKey`)
      (goto _label_2)
      (else
        (`self.ToggleDoor`)))))

(fn `getID`
  (returns (ID :type Integer))
  (return (`self._id`)))

(fn `UserConstructionScript`)