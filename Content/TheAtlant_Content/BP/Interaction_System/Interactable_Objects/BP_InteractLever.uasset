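; BP_InteractLever is an interactable lever that triggers a linked BP_InteractDoor.
; At BeginPlay it searches all doors in the level and stores the first one whose ID matches its own, marking itself linked.
; Interact and TakeDamage share the same path, which calls LeverPulled on that door if linked.
; A one-time-use flag limits the lever to a single pull, and debug prints report linking and interaction.
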(event `self.ReceiveBeginPlay`
  ;[1 0.4348 0.8352] Link lever to correct door
  (bind _outactors (`GameplayStatics.GetAllActorsOfClass` "/Game/TheAtlant_Content/BP/Interaction_System/Interactable_Objects/BP_InteractDoor.BP_InteractDoor_C"))
  (bind _returnvalue (`KismetArrayLibrary.Array_Length` _outactors))
  (if (> _returnvalue 0)
    (for _index (range _returnvalue)
      (bind _output (`|GetArrayItem` _outactors _index))
      (bind _id (`/Game/TheAtlant_Content/BP/Interaction_System/Interactable_Objects/BP_InteractDoor.getID` _output))
      (if (== _id (`self._id`))
        (set `self._doorRef` _output)
        (set `self._isLinked` true)
        (`KismetSystemLibrary.PrintString` "Linked to correct door" false)
        (break)))))

(event `self.Interact`
  ;[0.3903 0.8525 1] Interact
  (`KismetSystemLibrary.PrintText` "I am lever" :!label _label)
  (if (`self._isLinked`)
    (if (`self._isOneTimeUse`)
      (if (not (`self._used`))
        (set `self._used` true :!label _label_2)
        (`/Game/TheAtlant_Content/BP/Interaction_System/Interactable_Objects/BP_InteractDoor.LeverPulled` (`self._doorRef`)))
      (else
        (goto _label_2)))))

(event `/Game/TheAtlant_Content/BP/Shark/IA/BPI_Damageable.TakeDamage`
  ;[0.3903 0.8525 1] Interact
  (goto _label))

(fn `UserConstructionScript`)