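; Interactable lever that operates the double door sharing its ID, with optional one-time use.
; On BeginPlay it searches all BP_InteractDoorDouble actors for the matching ID and stores that door.
; Interacting plays the lever sound and calls LeverPulled on the linked door, unless a QTE is active.
; Taking damage launches a player QTE through an event dispatcher, with a hit-countdown handler that can also operate the lever.
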(event `self.ReceiveBeginPlay`
  ;[1 0.4348 0.8352] Link lever to correct door
  (bind _outactors (`GameplayStatics.GetAllActorsOfClass` "/Game/TheAtlant_Content/BP/Interaction_System/Interactable_Objects/BP_InteractDoorDouble.BP_InteractDoorDouble_C"))
  (bind _returnvalue (`KismetArrayLibrary.Array_Length` _outactors))
  (if (> _returnvalue 0)
    (for _index (range _returnvalue)
      (bind _output (`|GetArrayItem` _outactors _index))
      (bind _id (`/Game/TheAtlant_Content/BP/Interaction_System/Interactable_Objects/BP_InteractDoorDouble.getID` _output))
      (if (== _id (`self._id`))
        (set `self._doorRef` _output)
        (set `self._isLinked` true)
        (`KismetSystemLibrary.PrintString` "Linked to correct door" false)
        (break)))))

(event `CE_Operate`
  ;[0.3903 0.8525 1] Interact
  (if (not (`self.isInQTE`))
    (`KismetSystemLibrary.PrintText` "I am lever")
    (if (`self._isLinked`)
      (if (`self._isOneTimeUse`)
        (if (not (`self._used`))
          (set `self._used` true :!label _label)
          (`GameplayStatics.PlaySoundAtLocation` (`self.LeverSound`) (`SceneComponent.K2_GetComponentLocation` (`self.DefaultSceneRoot`)) (struct) 1.0 1.0 0.0 null null null null)
          (`/Game/TheAtlant_Content/BP/Interaction_System/Interactable_Objects/BP_InteractDoorDouble.LeverPulled` (`self._doorRef`)))
        (else
          (goto _label))))))

(event `self.Interact`
  ;[0.3903 0.8525 1] Interact
  (`self.CE_Operate`))

(event `self.TakeDamage`
  ;[1 1 1] QTE events
  (set `self.CurrentNumberHit` (`self.NumberHit`))
  (bind _asbp_player (cast `/Game/TheAtlant_Content/BP/BP_Player` (`GameplayStatics.GetPlayerCharacter` 0)))
  (`/Game/TheAtlant_Content/BP/BP_Player.ED_OnLaunchQTE` _asbp_player (`self.NumberHit`))
  (add `/Game/TheAtlant_Content/BP/BP_Player.ED_OnLaunchQTE` _asbp_player (`|CreateDelegate` :!event `CE_StopQTE`)))

(event `CE_StopQTE`
  (params (NumberHit :type Integer))
  (bind _currentnumberhit (`self.CurrentNumberHit`))
  ;[1 1 1] QTE events
  (if (not (> NumberHit 0))
    (`/Engine/EditorBlueprintResources/StandardMacros.DecrementInt` _currentnumberhit
      (:`  `
        (if (not (>= _currentnumberhit 0))
          (set `self.isInQTE` false)
          (`self.CE_Operate`))))))

(fn `UserConstructionScript`)