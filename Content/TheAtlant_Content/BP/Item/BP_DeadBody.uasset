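; Carryable dead body item, typed as Objective, Useless or Possessed, that the player picks up and drops.
; Objective and Useless bodies lose physics and collision and attach to the player's carry point when takeable.
; Picking up a Possessed body instead spawns a jellyfish that attacks the player, then the body becomes Useless and takeable after a short delay.
; Dropping detaches and places the body at the drop location, aligned to the player's yaw.
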(event `self.ReceiveBeginPlay`
  (`parent.ReceiveBeginPlay`)
  (set `self.IsDeadBody` true)
  ;[1 1 1] Can't take if possssed
  (switch `/Game/TheAtlant_Content/Data/Enum/E_DeadBodyTypes` (`self.Type`)
    (:`NewEnumerator2`
      (set `self.CanTake` false))))

(event `CE_PushBody`
  ;[1 1 1] Push dead body
  (bind _collision (`self.Collision`)
    (:`then`
      (`PrimitiveComponent.SetSimulatePhysics` _collision true)
      (`PrimitiveComponent.SetCollisionEnabled` _collision "QueryAndPhysics")
      (`PrimitiveComponent.AddForce` _collision (0.0 0.0 1000.0) "None" true))
    (:`else`)))

(event `self.CE_Pickup`
  (params (BP_Player :type "/Game/TheAtlant_Content/BP/BP_Player Object Reference"))
  ;[1 1 1] PickUp
  (switch `/Game/TheAtlant_Content/Data/Enum/E_DeadBodyTypes` (`self.Type`)
    (:`NewEnumerator0`
      (if (`self.CanTake`) :!label _label
        (bind _collision (`self.Collision`)
          (:`then`
            (`PrimitiveComponent.SetSimulatePhysics` _collision false)
            (`PrimitiveComponent.SetCollisionEnabled` _collision "NoCollision")
            (set `self.IsTaken` true)
            (set `/Game/TheAtlant_Content/BP/BP_Player.CarriedObject` self BP_Player)
            (if (`self.IsDeadBody`)
              (bind _deadbodypoint (`/Game/TheAtlant_Content/BP/BP_Player.DeadBodyPoint` BP_Player)
                (:`then`
                  (`self.K2_AttachToComponent` _deadbodypoint "None" "SnapToTarget" "SnapToTarget" "SnapToTarget"))
                (:`else`))
              (else
                (bind _itemcarrypoint (`/Game/TheAtlant_Content/BP/BP_Player.ItemCarryPoint` BP_Player)
                  (:`then`
                    (`self.K2_AttachToComponent` _itemcarrypoint "None" "SnapToTarget" "SnapToTarget" "SnapToTarget")
                    (bind _rotatingmovement (`self.RotatingMovement`)
                      (:`then`
                        (`ActorComponent.Activate` _rotatingmovement false))
                      (:`else`)))
                  (:`else`)))))
          (:`else`))))
    (:`NewEnumerator1`
      (goto _label))
    (:`NewEnumerator2`
      ;;[1 1 1] Spawn jelly fish if possessed
      (bind _returnvalue (`|SpawnActorFromClass` "/Game/TheAtlant_Content/BP/BP_JellyFish.BP_JellyFish_C" (`self.GetTransform`) "Undefined" "MultiplyWithRoot" null null))
      (`/Game/TheAtlant_Content/BP/BP_JellyFish.CE_AttackPlayer` _returnvalue BP_Player)
      (set `self.Type` "NewEnumerator1")
      ;;;[1 1 1] Wait for jelly to come out then can take
      (`KismetSystemLibrary.Delay` 1.0)
      (set `self.CanTake` true))))

(event `self.CE_Drop`
  (params (BP_Player :type "/Game/TheAtlant_Content/BP/BP_Player Object Reference") (DropLocation :type "Vector Structure"))
  (bind (_returnvalue_roll _returnvalue_pitch _returnvalue_yaw) (`KismetMathLibrary.BreakRotator` (`self.K2_GetActorRotation` BP_Player)))
  ;[1 1 1] Drop
  (`self.K2_DetachFromActor` "KeepWorld" "KeepWorld")
  (bind _collision (`self.Collision`)
    (:`then`
      (`PrimitiveComponent.SetCollisionEnabled` _collision "QueryOnly")
      (bind (_returnvalue_x _returnvalue_y _returnvalue_z) (`KismetMathLibrary.BreakVector` (`BoxComponent.GetScaledBoxExtent` _collision)))
      (`self.K2_SetActorLocation` (+ DropLocation (`KismetMathLibrary.MakeVector` 0.0 0.0 _returnvalue_z)))
      (`self.K2_SetActorRotation` (`KismetMathLibrary.MakeRotator` 0.0 0.0 _returnvalue_yaw))
      (bind _rotatingmovement (`self.RotatingMovement`)
        (:`then`
          (`ActorComponent.Deactivate` _rotatingmovement)
          (`self.CE_PushBody`))
        (:`else`)))
    (:`else`)))

(fn `DragEvent`
  (params (ActivateEvent :type Boolean))
  (returns (ShouldUnhook :type Boolean))
  (bind _collision (`self.Collision`)
    (:`then`
      (`PrimitiveComponent.SetPhysicsLinearVelocity` _collision (0.0 0.0 0.0) false "None")
      (return false))
    (:`else`)))

(fn `UserConstructionScript`
  (`parent.UserConstructionScript`))