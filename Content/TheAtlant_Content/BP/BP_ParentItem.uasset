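; Parent Blueprint for carryable items, including dead bodies, that the player can pick up and drop.
; Pickup registers the item as the player's CarriedObject, disables physics and collision, and attaches it to DeadBodyPoint or ItemCarryPoint, spinning non-body items via RotatingMovement.
; Drop detaches it, restores query-only collision, places it at the drop location raised by the box's half-height, matches the player's yaw and stops the spin.
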(event `self.ReceiveBeginPlay`
  ;[1 1 1] Deactivate rotation
  (bind _rotatingmovement (`self.RotatingMovement`)
    (:`then`
      (`ActorComponent.Deactivate` _rotatingmovement))
    (:`else`)))

(event `CE_Pickup`
  (params (BP_Player :type "/Game/TheAtlant_Content/BP/BP_Player Object Reference"))
  ;[1 1 1] Pickup Object
  (set `/Game/TheAtlant_Content/BP/BP_Player.CarriedObject` self BP_Player)
  ;;[1 1 1] Attach yourself to player
  (if (`self.IsDeadBody`)
    (bind _deadbodypoint (`/Game/TheAtlant_Content/BP/BP_Player.DeadBodyPoint` BP_Player)
      (:`then`
        (`self.K2_AttachToComponent` _deadbodypoint "None" "SnapToTarget" "KeepRelative" "SnapToTarget"))
      (:`else`))
    (else
      (bind _itemcarrypoint (`/Game/TheAtlant_Content/BP/BP_Player.ItemCarryPoint` BP_Player)
        (:`then`
          (`self.K2_AttachToComponent` _itemcarrypoint "None" "SnapToTarget" "SnapToTarget" "SnapToTarget")
          ;;[1 1 1] Activate Rotation if item
          (bind _rotatingmovement (`self.RotatingMovement`)
            (:`then`
              (`ActorComponent.Activate` _rotatingmovement false))
            (:`else`)))
        (:`else`))))
  ;;[1 1 1] Disable collision
  (bind _collision (`self.Collision`)
    (:`then`
      (`PrimitiveComponent.SetSimulatePhysics` _collision false)
      (`PrimitiveComponent.SetCollisionEnabled` _collision "NoCollision"))
    (:`else`)))

(event `CE_Drop`
  (params (BP_Player :type "/Game/TheAtlant_Content/BP/BP_Player Object Reference") (DropLocation :type "Vector Structure"))
  (bind (_returnvalue_roll _returnvalue_pitch _returnvalue_yaw) (`KismetMathLibrary.BreakRotator` (`self.K2_GetActorRotation` BP_Player)))
  ;[1 1 1] Drop Object
  (`self.K2_DetachFromActor` "KeepWorld" "KeepWorld")
  (bind _collision (`self.Collision`)
    (:`then`
      (`PrimitiveComponent.SetCollisionEnabled` _collision "QueryOnly")
      (bind (_returnvalue_x _returnvalue_y _returnvalue_z) (`KismetMathLibrary.BreakVector` (`BoxComponent.GetScaledBoxExtent` _collision)))
      (`self.K2_SetActorLocation` (+ DropLocation (`KismetMathLibrary.MakeVector` 0.0 0.0 _returnvalue_z)))
      (`self.K2_SetActorRotation` (`KismetMathLibrary.MakeRotator` 0.0 0.0 _returnvalue_yaw))
      (bind _rotatingmovement (`self.RotatingMovement`)
        (:`then`
          (`ActorComponent.Deactivate` _rotatingmovement))
        (:`else`)))
    (:`else`)))

(fn `UserConstructionScript`)