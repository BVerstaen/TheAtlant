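; Pufferfish hazard that swells when an actor enters its collision and explodes at full swell, damaging the player.
; A timeline lerps mesh scale and height alongside the puff animation, reversing if the actor leaves or becomes invalid, then resuming the looping swim animation.
; A completed swell calls the player's hit event, spawns a Niagara explosion and destroys the fish.
; MetaSound triggers voice puff up, puff down and explosion, fading out opposing puff sounds.
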(event `self.ReceiveBeginPlay`
  ;[1 1 1] Set default scale & Z position
  (bind _smesh (`self.SMesh`)
    (:`then`
      (bind _relativescale3d_x (`KismetMathLibrary.BreakVector` (`SceneComponent.RelativeScale3D` _smesh)))
      (set `self.DefaultScale` _relativescale3d_x)
      (bind (_relativelocation_x _relativelocation_y _relativelocation_z) (`KismetMathLibrary.BreakVector` (`SceneComponent.RelativeLocation` _smesh)))
      (set `self.DefaultZPosition` _relativelocation_z))
    (:`else`)))

(event `CE_StopTimeline`
  (bind _defaultzposition (`self.DefaultZPosition`))
  ;[1 1 1] Swelling & Explosion
  (bind (_direction _swellinglerp) (`Timeline|tl_Swelling` :!via `Stop` :!label _label)
    (:`Update`
      (bind _smesh (`self.SMesh`)
        (:`then`
          (bind _returnvalue (`KismetMathLibrary.Lerp` (`self.DefaultScale`) (`self.SwellScale`) _swellinglerp))
          (`SceneComponent.SetRelativeScale3D` _smesh (`KismetMathLibrary.MakeVector` _returnvalue _returnvalue _returnvalue))
          (`SceneComponent.K2_SetRelativeLocation` _smesh (`KismetMathLibrary.MakeVector` 0.0 0.0 (`KismetMathLibrary.Lerp` _defaultzposition (+ _defaultzposition -40.0) _swellinglerp)) false false)
          ;;[1 1 1] If player died, stop swelling & dereference player
          (`self.PlayerActor`
            (:`then`)
            (:`else`
              (set `self.PlayerActor` null)
              (bind _smesh_2 (`self.SMesh`)
                (:`then`
                  (`SkeletalMeshComponent.SetPlayRate` _smesh_2 -1.0)
                  (goto _label :!via `Reverse`))
                (:`else`)))))
        (:`else`)))
    (:`Finished`
      ;;[1 1 1] Destroy & spawn effect & damage actor
      ;;;[1 1 1] Look if finish from forward
      (switch `ETimelineDirection` _direction
        (:`Forward`
          (set `self.HasExploded` true)
          ;;;[1 1 1] Deal damage
          (bind _playeractor (`self.PlayerActor`)
            (:`then`
              (bind _asbp_player (cast `/Game/TheAtlant_Content/BP/BP_Player` _playeractor))
              (`/Game/TheAtlant_Content/BP/BP_Player.CE_PlayerHit` _asbp_player 1)
              ;;;[1 1 1] Spawn effect
              (bind _collision (`self.Collision`)
                (:`then`
                  (`NiagaraFunctionLibrary.SpawnSystemAtLocation` "/Game/TheAtlant_Content/VFX/NS_FuguExplosion.NS_FuguExplosion" (`SceneComponent.K2_GetComponentLocation` _collision) (`SceneComponent.K2_GetComponentRotation` _collision))
                  (`self.FuguBoom`)
                  (`self.K2_DestroyActor`))
                (:`else`)))
            (:`else`)))
        (:`Backward`
          ;;;[1 1 1] Reset animation
          (bind _smesh_3 (`self.SMesh`)
            (:`then`
              (`SkeletalMeshComponent.PlayAnimation` _smesh_3 "/Game/TheAtlant_Content/GA/Fugu/fugu_version_finale/Animations/anim_nage_fugu.anim_nage_fugu" true)
              (`self.CE_StopTimeline`))
            (:`else`)))))))

(event `self.Collision.OnComponentBeginOverlap`
  (params (OverlappedComponent :type "PrimitiveComponent Object Reference") (OtherActor :type "Actor Object Reference") (OtherComp :type "PrimitiveComponent Object Reference") (OtherBodyIndex :type Integer) (bFromSweep :type Boolean) (SweepResult :type "HitResult Structure (by ref)"))
  ;[1 1 1] Swelling & Explosion
  ;;[1 1 1] Look if is player
  (`self.PlayerActor`
    (:`then`)
    (:`else`
      (set `self.PlayerActor` OtherActor)
      ;;[1 1 1] Set play rate
      (bind _smesh (`self.SMesh`)
        (:`then`
          (`SkeletalMeshComponent.SetPlayRate` _smesh 1.0)
          (`SkeletalMeshComponent.PlayAnimation` _smesh "/Game/TheAtlant_Content/GA/Fugu/fugu_version_finale/Animations/anim_gonfle_fugu.anim_gonfle_fugu" false)
          (`self.FuguPuffUp`)
          (goto _label))
        (:`else`)))))

(event `self.Collision.OnComponentEndOverlap`
  (params (OverlappedComponent :type "PrimitiveComponent Object Reference") (OtherActor :type "Actor Object Reference") (OtherComp :type "PrimitiveComponent Object Reference") (OtherBodyIndex :type Integer))
  ;[1 1 1] Swelling & Explosion
  ;;[1 1 1] Look if is player
  (if (`self.HasExploded`)
    _
    (elif (== OtherActor (`self.PlayerActor`))
      (set `self.PlayerActor` null)
      ;;[1 1 1] Set play rate
      (bind _smesh (`self.SMesh`)
        (:`then`
          (`SkeletalMeshComponent.SetPlayRate` _smesh -1.0)
          (`self.FuguPuffDown`)
          (goto _label :!via `Reverse`))
        (:`else`)))))

(event `/Game/TheAtlant_Content/BP/Shark/IA/BPI_Damageable.TakeDamage`
  ;[1 1 1] Swelling & Explosion
)

(event `FuguBoom`
  ;[1 0.581 0.966] Sounds
  (bind _returnvalue (`GameplayStatics.SpawnSoundAtLocation` "/Game/TheAtlant_Content/Audio/_MetaSounds/Pufferfish/MS_Pufferfish.MS_Pufferfish" (`SceneComponent.K2_GetComponentLocation` (`self.SMesh`)) (struct) 1.0 1.0 0.0 null null))
  (`AudioParameterControllerInterface.SetTriggerParameter` _returnvalue "Explode")
  (if (`KismetSystemLibrary.IsValid` (stale `FuguPuffDown` _returnvalue))
    (`AudioComponent.Stop` (stale `FuguPuffDown` _returnvalue))
    (if (`KismetSystemLibrary.IsValid` (stale `FuguPuffUp` _returnvalue))
      (`AudioComponent.Stop` (stale `FuguPuffUp` _returnvalue)))))

(event `FuguPuffUp`
  ;[1 0.581 0.966] Sounds
  (bind _returnvalue (`GameplayStatics.SpawnSoundAtLocation` "/Game/TheAtlant_Content/Audio/_MetaSounds/Pufferfish/MS_Pufferfish.MS_Pufferfish" (`SceneComponent.K2_GetComponentLocation` (`self.SMesh`)) (struct) 1.0 1.0 0.0 null null))
  (`AudioParameterControllerInterface.SetTriggerParameter` _returnvalue "Puff up")
  (if (`KismetSystemLibrary.IsValid` (stale `FuguPuffDown` _returnvalue))
    (`AudioComponent.FadeOut` (stale `FuguPuffDown` _returnvalue) 0.5 0.0 "Linear")))

(event `FuguPuffDown`
  ;[1 0.581 0.966] Sounds
  (bind _returnvalue (`GameplayStatics.SpawnSoundAtLocation` "/Game/TheAtlant_Content/Audio/_MetaSounds/Pufferfish/MS_Pufferfish.MS_Pufferfish" (`SceneComponent.K2_GetComponentLocation` (`self.SMesh`)) (struct) 1.0 1.0 0.0 null null))
  (`AudioParameterControllerInterface.SetTriggerParameter` _returnvalue "Puff down")
  (if (`KismetSystemLibrary.IsValid` (stale `FuguPuffUp` _returnvalue))
    (`AudioComponent.FadeOut` (stale `FuguPuffUp` _returnvalue) 0.5 0.0 "Linear")))

(fn `UserConstructionScript`)