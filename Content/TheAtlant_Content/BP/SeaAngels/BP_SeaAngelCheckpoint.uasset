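; Sea angel checkpoint actor that forms a linked path node for BP_SeaAngel to follow.
; On overlap with a sea angel, it sets the angel's FirstCheckPoint to its NextPoint, or calls CEFinishPath when no next point exists.
; Debug magenta lines to NextPoint are drawn in the construction script and every Tick, showing the chain in editor and at runtime.
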(event `self.ReceiveActorBeginOverlap`
  (params (OtherActor :type "Actor Object Reference"))
  ;[1 1 1] Pass to next target OR stop Path
  (bind _asbp_sea_angel (cast `/Game/TheAtlant_Content/BP/SeaAngels/BP_SeaAngel` OtherActor))
  (bind _nextpoint (`self.NextPoint`)
    (:`then`
      (set `/Game/TheAtlant_Content/BP/SeaAngels/BP_SeaAngel.FirstCheckPoint` _nextpoint _asbp_sea_angel))
    (:`else`
      (`/Game/TheAtlant_Content/BP/SeaAngels/BP_SeaAngel.CE_FinishPath` _asbp_sea_angel))))

(event `self.ReceiveTick`
  (params (DeltaSeconds :type "Float (single-precision)"))
  ;[1 1 1] DEBUG draw line
  (bind _nextpoint (`self.NextPoint`)
    (:`then`
      (`KismetSystemLibrary.DrawDebugLine` (`self.K2_GetActorLocation`) (`self.K2_GetActorLocation` _nextpoint) (struct :`R` 1.0 :`B` 0.891561 :`A` 1.0) 0.0 1.0))
    (:`else`)))

(fn `UserConstructionScript`
  ;[1 1 1] DEBUG draw line
  (bind _nextpoint (`self.NextPoint`)
    (:`then`
      (`KismetSystemLibrary.DrawDebugLine` (`self.K2_GetActorLocation`) (`self.K2_GetActorLocation` _nextpoint) (struct :`R` 1.0 :`B` 0.997784 :`A` 1.0) 0.1 1.0))
    (:`else`)))