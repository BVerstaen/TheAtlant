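; BP_SeaAngel is a sea angel actor that shows a spoken message on the HUD, then optionally swims toward a checkpoint.
; CallEvent triggers speech; after the message delay, a timeline eases rotation toward FirstCheckPoint and drives FloatingPawnMovement forward until CE_FinishPath stops it.
; An optional sphere trace just ahead withholds movement when it hits WorldStatic.
; Tick replays idle sounds after random delays, gated by the audio-finished callback.
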(event `/Game/TheAtlant_Content/BP/Event_system/BPI_EventFunctions.CallEvent`
  (`KismetSystemLibrary.PrintString` "Event ON")
  (`self.CE_Speaking` true))

(event `self.ReceiveBeginPlay`
  ;[1 1 1] Set default collision
  (if (`self.ShouldRemoveCollision`)
    (bind _cube (`self.Cube`)
      (:`then`
        (`PrimitiveComponent.SetCollisionEnabled` _cube "NoCollision"))
      (:`else`))))

(event `CE_Speaking`
  (params (ShouldMove :type Boolean) (AlternateMessage :type String))
  (bind _speakingtime (`self.SpeakingTime`))
  ;[1 1 1] Speaking (display message) then Start Path
  ;;[1 1 1] Change Speaking text if alternate message
  (if (!= AlternateMessage "")
    (set `self.SpeakingText` AlternateMessage))
  (bind _ashud_the_atlant (cast `/Game/TheAtlant_Content/BP/Game/HUD_TheAtlant` (`PlayerController.GetHUD` (`GameplayStatics.GetPlayerController` 0))))
  (`/Game/TheAtlant_Content/BP/Game/HUD_TheAtlant.CE_DisplayMessage` _ashud_the_atlant (`self.SpeakingText`) (`self.SpeakingColor`) _speakingtime)
  (`KismetSystemLibrary.Delay` _speakingtime)
  (if ShouldMove
    (`self.CE_StartPath`)))

(event `CE_StartPath`
  (bind _returnvalue (+ (`self.K2_GetActorLocation`) (* (`KismetMathLibrary.GetForwardVector` (`self.K2_GetActorRotation`)) 30.0)))
  ;[1 1 1] Path
  (`Timeline|tl_MoveCheckPoint` :!label _label
    (:`Update`
      ;;[1 1 1] Rotate to point
      (bind _firstcheckpoint (`self.FirstCheckPoint`)
        (:`then`
          (`self.K2_SetActorRotation` (`KismetMathLibrary.RInterpTo` (`self.K2_GetActorRotation`) (`KismetMathLibrary.FindLookAtRotation` (`self.K2_GetActorLocation`) (`self.K2_GetActorLocation` _firstcheckpoint)) (`GameplayStatics.GetWorldDeltaSeconds`) (`self.RotateSpeed`)))
          ;;[1 1 1] Look if there's a wall in front
          (bind (_outhit _returnvalue_2) (`KismetSystemLibrary.SphereTraceSingleForObjects` _returnvalue _returnvalue 10.0 (`|MakeArray` "ObjectTypeQuery1" :!type "EObjectTypeQuery Enum")))
          (if (not (and (`self.ShouldCheckForCollision`) _returnvalue_2))
            ;;[1 1 1] Move to position
            (bind _floatingpawnmovement (`self.FloatingPawnMovement`)
              (:`then`
                (set `MovementComponent.Velocity` (* (`self.MoveSpeed`) (`self.GetActorForwardVector`)) _floatingpawnmovement))
              (:`else`))))
        (:`else`)))))

(event `CE_FinishPath`
  ;[1 1 1] Path
  (goto _label :!via `Stop`))

(event `self.ReceiveTick`
  (params (DeltaSeconds :type "Float (single-precision)"))
  (bind _idlesounds (`self.IdleSounds`))
  ;[0.3047 1 0.6059] Idle Sounds
  (if (not (`self.AudioPlaying`))
    (set `self.AudioPlaying` true)
    (`KismetSystemLibrary.Delay` (`KismetMathLibrary.RandomFloatInRange` (`self.MinAudioDelay`) (`self.MaxAudioDelay`)))
    (`AudioComponent.Play` _idlesounds 0.0)
    (add `AudioComponent.OnAudioFinished` _idlesounds (delegate `OnAudioFinished`))))

(event `OnAudioFinished`
  ;[0.3047 1 0.6059] Idle Sounds
  (set `self.AudioPlaying` false))

(fn `UserConstructionScript`)