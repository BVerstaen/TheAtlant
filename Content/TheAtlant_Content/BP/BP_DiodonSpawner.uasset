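; Spawner actor that populates its Collision box with BP_Diodon (fugu) actors on BeginPlay, as many as NumberOfDiodon.
; Each spawn tries random unit vectors scaled by the box extent, keeping the first spot where a zero-length Visibility sphere trace hits nothing.
; Accepted spots spawn a diodon with random yaw; exhausted retries print a warning for designers.
; The construction script resets a negative count to one.
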(event `self.ReceiveBeginPlay`
  (for _ (range (`self.NumberOfDiodon`))
    (`self.SpawnOneFugu`)))

(fn `SpawnOneFugu`
  (locals (NewPosition :type "Vector Structure") (CorrectPosition :type Boolean) (NewFugu :type "/Game/TheAtlant_Content/BP/BP_Diodon Object Reference") (SphereRadius :type "Float (double-precision)" :default 32.0))
  (for _ (range 11)
    ;[1 1 1] Find Random spot
    (bind _collision (`self.Collision`)
      (:`then`
        (bind _output_get (set `local.NewPosition` (* (`KismetMathLibrary.RandomUnitVector`) (`BoxComponent.GetScaledBoxExtent` _collision))))
        (bind _returnvalue (+ _output_get (`SceneComponent.K2_GetComponentLocation` _collision)))
        ;[1 1 1] Test random spot
        (bind (_outhit _returnvalue_2) (`KismetSystemLibrary.SphereTraceSingle` _returnvalue _returnvalue (`local.SphereRadius`) "TraceTypeQuery1"))
        (bind _output_get_2 (set `local.CorrectPosition` (not _returnvalue_2)))
        (if _output_get_2
          ;;[1 1 1] Spawn the fugu
          (bind _collision_2 (`self.Collision`)
            (:`then`
              (`|SpawnActorFromClass` "/Game/TheAtlant_Content/BP/BP_Diodon.BP_Diodon_C" (`KismetMathLibrary.MakeTransform` (+ (`SceneComponent.K2_GetComponentLocation` _collision_2) (`local.NewPosition`)) (`KismetMathLibrary.MakeRotator` 0.0 0.0 (`KismetMathLibrary.RandomFloatInRange` 0.0 360.0))) "Undefined" "MultiplyWithRoot" null null)
              (break))
            (:`else`))))
      (:`else`)))
  ;[1 1 1] If can't find valid spot -> harrass GD
  (if (not (`local.CorrectPosition`))
    (`KismetSystemLibrary.PrintString` "Can't find a valid position for diodon, mesh is too big / too many meshs in same BP_Diodon" true true (struct :`R` 1.0 :`B` 0.017012 :`A` 1.0)))
  (return))

(fn `UserConstructionScript`
  (if (< (`self.NumberOfDiodon`) 0)
    (set `self.NumberOfDiodon` 1)))