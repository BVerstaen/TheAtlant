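; BP_CurrentTrap is an interactable trap door that turns a water current on when open and off when closed.
; Interact toggles IsOpened and plays or reverses a timeline that pitches RotatePoint between closed and open.
; When the timeline finishes, its direction decides whether a BP_WaterCurrent is spawned at WaterCurrentSpawnPoint or the existing one is destroyed.
; BeginPlay snaps the door to its initial IsOpened state, creating the current immediately if open.
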(event `self.ReceiveBeginPlay`
  (bind _rotatepoint (`self.RotatePoint`)
    (:`then`
      (if (`self.IsOpened`)
        (`SceneComponent.K2_SetRelativeRotation` _rotatepoint (`KismetMathLibrary.MakeRotator` 0.0 90.0) false false)
        (`self.CE_CreateWaterCurrent`)
        (else
          (`SceneComponent.K2_SetRelativeRotation` _rotatepoint (`KismetMathLibrary.MakeRotator` 0.0 0.0) false false))))
    (:`else`)))

(event `/Game/TheAtlant_Content/BP/Interaction_System/BPI_InteractableObject.Interact`
  ;[1 1 1] Interaction
  (bind _output_get (set `self.IsOpened` (not (`self.IsOpened`))))
  (if _output_get
    ;[1 1 1] Rotation Animation
    (bind (_direction _rotationlerp) (`Timeline|tl_TrapDoorAnimation` :!label _label)
      (:`Update`
        (bind _rotatepoint (`self.RotatePoint`)
          (:`then`
            (`SceneComponent.K2_SetRelativeRotation` _rotatepoint (`KismetMathLibrary.MakeRotator` 0.0 (`KismetMathLibrary.Lerp` 0.0 90.0 _rotationlerp)) false false))
          (:`else`)))
      (:`Finished`
        ;;[1 1 1] Create / destroy the water current
        (switch `ETimelineDirection` _direction
          (:`Forward`
            (`self.CE_CreateWaterCurrent`))
          (:`Backward`
            (`self.CE_DestroyWaterCurrent`)))))
    (else
      (goto _label :!via `Reverse`))))

(event `CE_CreateWaterCurrent`
  ;[1 1 1] Create / Destroy the water current
  (`self.WaterCurrentActor`
    (:`then`)
    (:`else`
      (bind _watercurrentspawnpoint (`self.WaterCurrentSpawnPoint`)
        (:`then`
          (bind _returnvalue (`|SpawnActorFromClass` "/Game/TheAtlant_Content/BP/BP_WaterCurrent.BP_WaterCurrent_C" (`SceneComponent.K2_GetComponentToWorld` _watercurrentspawnpoint) "Undefined" "MultiplyWithRoot" null null))
          (set `self.WaterCurrentActor` _returnvalue))
        (:`else`)))))

(event `CE_DestroyWaterCurrent`
  ;[1 1 1] Create / Destroy the water current
  (bind _watercurrentactor (`self.WaterCurrentActor`)
    (:`then`
      (`self.K2_DestroyActor` _watercurrentactor))
    (:`else`)))

(fn `UserConstructionScript`)