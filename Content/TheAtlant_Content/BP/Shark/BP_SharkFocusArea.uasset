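; BP_SharkFocusArea is a trigger area that makes its linked shark focus on the player.
; On actor overlap, it calls CEFocusPlayer on LinkedShark if the actor is a BP_Player not in a hide area and the shark reference is valid.
; Each tick it runs a box trace matching the Collision extent with one-frame debug drawing, but the trace result is unused.
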(event `self.ReceiveActorBeginOverlap`
  (params (OtherActor :type "Actor Object Reference"))
  (bind _asbp_player (cast `/Game/TheAtlant_Content/BP/BP_Player` OtherActor))
  (if (not (`/Game/TheAtlant_Content/BP/BP_Player.IsInHideArea` _asbp_player))
    (bind _linkedshark (`self.LinkedShark`)
      (:`then`
        (`/Game/TheAtlant_Content/BP/Shark/BP_Shark.CE_FocusPlayer` _linkedshark))
      (:`else`))))

(event `self.ReceiveTick`
  (params (DeltaSeconds :type "Float (single-precision)"))
  (bind _returnvalue (`self.K2_GetActorLocation`))
  (bind _collision (`self.Collision`)
    (:`then`
      (`KismetSystemLibrary.BoxTraceSingleForObjects` :`Start` _returnvalue :`End` _returnvalue :`HalfSize` (`BoxComponent.BoxExtent` _collision) :`Orientation` (`self.K2_GetActorRotation`) :`ObjectTypes` (`|MakeArray` "ObjectTypeQuery7" :!type "EObjectTypeQuery Enum") :`DrawDebugType` "ForOneFrame"))
    (:`else`)))

(fn `UserConstructionScript`)