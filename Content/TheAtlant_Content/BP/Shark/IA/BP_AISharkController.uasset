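; AI controller for the shark, which runs its behavior tree on possess and drives patrol, chase and flee through Blackboard keys.
; Each tick, a sphere trace along the shark's forward vector, sized by its sight settings, flags a living player as the chase target.
; A harpoon hit clears that target and sets a run-away point from the shark's patrol area.
; Losing sight happens only by event, not by a failed trace.
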(event `self.ReceivePossess`
  (params (PossessedPawn :type "Pawn Object Reference"))
  ;[1 1 1] Set IA Controller & Run Behaviour Tree
  (bind _asbp_shark (cast `/Game/TheAtlant_Content/BP/Shark/BP_Shark` PossessedPawn))
  (bind _output_get (set `self.BP_Shark` _asbp_shark))
  (set `/Game/TheAtlant_Content/BP/Shark/BP_Shark.BP_AIController` self _output_get)
  (`self.RunBehaviorTree` "/Game/TheAtlant_Content/BP/Shark/IA/BT_Shark.BT_Shark"))

(event `self.ReceiveTick`
  (params (DeltaSeconds :type "Float (single-precision)"))
  ;[1 1 1] Look for player
  (bind _bp_shark (`self.BP_Shark`)
    (:`then`
      (bind _returnvalue (`self.K2_GetActorLocation` _bp_shark))
      (bind (_outhit _returnvalue_2) (`KismetSystemLibrary.SphereTraceSingleForObjects` :`Start` _returnvalue :`End` (+ _returnvalue (* (`self.GetActorForwardVector` _bp_shark) (`/Game/TheAtlant_Content/BP/Shark/BP_Shark.SeeDistance` _bp_shark))) :`Radius` (`/Game/TheAtlant_Content/BP/Shark/BP_Shark.SeeRadius` _bp_shark) :`ObjectTypes` (`|MakeArray` "ObjectTypeQuery1" "ObjectTypeQuery7" "ObjectTypeQuery10" :!type "EObjectTypeQuery Enum") :`DrawDebugType` "ForOneFrame"))
      ;;[1 1 1] Look if found alive player
      (if _returnvalue_2
        (bind _asbp_player (cast `/Game/TheAtlant_Content/BP/BP_Player` (`.HitActor` (`GameplayStatics.BreakHitResult` _outhit))))
        (set `self.ActorSeen` _asbp_player)
        (if (> (`/Game/TheAtlant_Content/BP/BP_Player.HealthPoints` _asbp_player) 0)
          ;;[1 1 1] go into chase mode
          (bind _blackboard (`self.Blackboard`)
            (:`then`
              (`BlackboardComponent.SetValueAsBool` _blackboard (`self.HasLineOfSight`) true)
              (`BlackboardComponent.SetValueAsBool` _blackboard (`self.HasLineOfSight`) true)
              (`BlackboardComponent.SetValueAsObject` _blackboard (`self.PlayerActor`) (`self.ActorSeen`))
              (`KismetSystemLibrary.PrintString` "Got player"))
            (:`else`)))))
    (:`else`)))

(event `CE_Hit`
  ;[1 1 1] Hit by harpoon
  (`self.CE_LosePlayerSight`)
  ;;[1 1 1] Set run away state & point
  (bind _blackboard (`self.Blackboard`)
    (:`then`
      (`BlackboardComponent.SetValueAsBool` _blackboard (`self.IsRunningAway`) true)
      (bind _bp_shark (`self.BP_Shark`)
        (:`then`
          (bind _bp_patrolarea (`/Game/TheAtlant_Content/BP/Shark/BP_Shark.BP_PatrolArea` _bp_shark)
            (:`then`
              (bind _point (`/Game/TheAtlant_Content/BP/Shark/BP_SharkPatrolArea.GiveRunAwayPoint` _bp_patrolarea))
              (`BlackboardComponent.SetValueAsVector` _blackboard (`self.RunAwayPosition`) _point)
              (`BlackboardComponent.ClearValue` _blackboard (`self.PatrolPoint`)))
            (:`else`)))
        (:`else`)))
    (:`else`)))

(event `CE_LosePlayerSight`
  ;[1 1 1] Lose player sight
  (bind _blackboard (`self.Blackboard`)
    (:`then`
      (`BlackboardComponent.SetValueAsBool` _blackboard (`self.HasLineOfSight`) false)
      (`BlackboardComponent.SetValueAsObject` _blackboard (`self.PlayerActor`) null))
    (:`else`)))

(fn `UserConstructionScript`)