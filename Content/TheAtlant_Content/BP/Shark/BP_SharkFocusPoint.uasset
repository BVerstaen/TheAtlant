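; BP_SharkFocusPoint is an actor that redirects a linked shark to its own location, intended for when a linked corpse is taken.
; BeginPlay only prints warnings for an invalid corpse or shark.
; CE_SharkFocusPoint clears the shark's IsRunningAway and HasLineOfSight blackboard keys and sets CurrentPatrolLocation to the actor's position.
; The timeline polling the corpse's IsTaken flag is never started, so nothing here triggers that event.
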(event `self.ReceiveBeginPlay`
  ;[1 1 1] Check valid setup
  (`self.LinkedCorpse`
    (:`then`
      (`self.LinkedShark`
        (:`then`)
        (:`else`
          (`KismetSystemLibrary.PrintString` "Invalid Shark"))))
    (:`else`
      (`KismetSystemLibrary.PrintString` "Invalid Corpse"))))

(event `CE_SharkFocusPoint`
  ;[1 1 1] Set shark point
  (bind _linkedshark (`self.LinkedShark`)
    (:`then`
      (bind _returnvalue (`AIBlueprintHelperLibrary.GetBlackboard` _linkedshark))
      (`BlackboardComponent.SetValueAsBool` _returnvalue "IsRunningAway" false)
      (`BlackboardComponent.SetValueAsBool` _returnvalue "HasLineOfSight" false)
      (`BlackboardComponent.SetValueAsVector` _returnvalue "CurrentPatrolLocation" (`self.K2_GetActorLocation`)))
    (:`else`)))

(fn `UserConstructionScript`)