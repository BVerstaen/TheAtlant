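; Breakable porthole (hublot) for the scripted shark content, which shatters after a set number of hits.
; BreakCheck decrements the remaining hit count, fires the break event at zero or below and returns whether it broke.
; Breaking spawns a master field at the actor to fracture the glass and plays a random destruction sound.
; It then destroys the field's root component and starts a timer that removes the actor once the shatter duration ends.
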(event `self.ReceiveBeginPlay`
  (`parent.ReceiveBeginPlay`))

(event `CE_Break`
  (bind _sound (`self.Sound`))
  ;[1 1 1] Break glass
  (bind _returnvalue (`|SpawnActorFromClass` "/Engine/EditorResources/FieldNodes/FS_MasterField.FS_MasterField_C" (`self.GetTransform`) "Undefined" "MultiplyWithRoot" null null))
  ;;[1 0.3795 0.9821] Sound destroy
  (`KismetArrayLibrary.Array_Shuffle` _sound)
  (`GameplayStatics.PlaySoundAtLocation` (`|GetArrayItem` _sound) (`SceneComponent.K2_GetComponentLocation` (`self.GC_BP_Hublot`)) (struct) 1.0 1.0 0.0 null null null null)
  (bind _rootcomponent (`Actor.RootComponent` _returnvalue)
    (:`then`
      (`ActorComponent.K2_DestroyComponent` _rootcomponent)
      (`KismetSystemLibrary.K2_SetTimerDelegate` (delegate `CE_Destroy`) (`self.ShattersDuration`)))
    (:`else`)))

(event `CE_Destroy`
  ;[1 1 1] Break glass
  (`self.K2_DestroyActor`))

(fn `BreakCheck`
  (returns (IsBroken :type Boolean))
  (bind _result (`/Engine/EditorBlueprintResources/StandardMacros.DecrementInt` (`self.NumberHit`))
    (:`  `
      (bind _returnvalue (<= _result 0))
      (if _returnvalue
        (`self.CE_Break`))
      (return _returnvalue))))

(fn `UserConstructionScript`
  (`parent.UserConstructionScript`))