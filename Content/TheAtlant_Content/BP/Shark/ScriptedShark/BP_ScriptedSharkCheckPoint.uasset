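; BP_ScriptedSharkCheckPoint is a chained waypoint that steers a BP_ScriptedShark along a scripted path.
; On overlap, its NextAction either stops the shark, sends it to NextPoint with optional new speeds, or switches it to AI.
; The AI switch stops the path, then hands over LinkedPatrolArea with player-focus and never-forget options.
; Tick and the construction script draw debug lines to the next point.
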(event `self.ReceiveActorBeginOverlap`
  (params (OtherActor :type "Actor Object Reference"))
  (bind _newmovespeed (`self.NewMoveSpeed`))
  (bind _newrotatespeed (`self.NewRotateSpeed`))
  ;[1 1 1] Pass to next target OR stop Path
  (bind _asbp_scripted_shark (cast `/Game/TheAtlant_Content/BP/Shark/ScriptedShark/BP_ScriptedShark` OtherActor))
  (switch `/Game/TheAtlant_Content/BP/Shark/ScriptedShark/E_SSNextAction` (`self.NextAction`)
    (:`NewEnumerator1`
      (`/Game/TheAtlant_Content/BP/Shark/ScriptedShark/BP_ScriptedShark.CE_StopPath` _asbp_scripted_shark))
    (:`NewEnumerator4`
      ;;[1 1 1] Move to next checkpoint
      (bind _nextpoint (`self.NextPoint` :!label _label)
        (:`then`
          (set `/Game/TheAtlant_Content/BP/Shark/ScriptedShark/BP_ScriptedShark.FirstCheckPoint` _nextpoint _asbp_scripted_shark))
        (:`else`
          (`/Game/TheAtlant_Content/BP/Shark/ScriptedShark/BP_ScriptedShark.CE_StopPath` _asbp_scripted_shark))))
    (:`NewEnumerator6`
      (if (not (== _newmovespeed 0.0))
        (set `/Game/TheAtlant_Content/BP/Shark/ScriptedShark/BP_ScriptedShark.MoveSpeed` _newmovespeed _asbp_scripted_shark))
      (if (== _newrotatespeed 0.0)
        (goto _label)
        (else
          (set `/Game/TheAtlant_Content/BP/Shark/ScriptedShark/BP_ScriptedShark.RotateSpeed` _newrotatespeed _asbp_scripted_shark)
          (goto _label))))
    (:`NewEnumerator0`
      (`self.M_SwitchIA` _asbp_scripted_shark))
    (:`NewEnumerator2`
      (`self.M_SwitchIA` _asbp_scripted_shark true))
    (:`NewEnumerator5`
      (`self.M_SwitchIA` _asbp_scripted_shark true true))))

(event `self.ReceiveTick`
  (params (DeltaSeconds :type "Float (single-precision)"))
  ;[1 1 1] DEBUG draw line
  (bind _nextpoint (`self.NextPoint`)
    (:`then`
      (`KismetSystemLibrary.DrawDebugLine` (`self.K2_GetActorLocation`) (`self.K2_GetActorLocation` _nextpoint) (struct :`R` 1.0 :`B` 0.891561 :`A` 1.0) 0.0 1.0))
    (:`else`)))

(fn `UserConstructionScript`
  (bind _nextpoint (`self.NextPoint`)
    (:`then`
      (`KismetSystemLibrary.DrawDebugLine` (`self.K2_GetActorLocation`) (`self.K2_GetActorLocation` _nextpoint) (struct :`R` 1.0 :`B` 0.997784 :`A` 1.0) 0.1 1.0))
    (:`else`)))