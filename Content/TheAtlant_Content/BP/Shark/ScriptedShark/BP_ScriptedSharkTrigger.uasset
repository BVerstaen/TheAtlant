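; One-shot overlap trigger that starts the behavior of a linked scripted shark.
; The first overlap by any actor fires an OnActivate dispatcher, then runs the selected first action: start the shark's path or switch it to AI, optionally focusing the player immediately.
; The AI switch passes the linked patrol area to the shark and is skipped if that area is invalid.
; BeginPlay logs a missing shark link.
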(event `self.ReceiveBeginPlay`
  ;[1 1 1] Check if valid shark
  (`self.LinkedScriptedShark`
    (:`then`)
    (:`else`
      (`KismetSystemLibrary.PrintString` "Invalid Shark" false))))

(event `self.ReceiveActorBeginOverlap`
  (params (OtherActor :type "Actor Object Reference"))
  ;[1 1 1] Start AI trigger
  (if (not (`self.WasActivated`))
    (set `self.WasActivated` true)
    (`self.ED_OnActivate`)
    (bind _linkedscriptedshark (`self.LinkedScriptedShark`)
      (:`then`
        (switch `/Game/TheAtlant_Content/BP/Shark/ScriptedShark/E_SSNextAction` (`self.FirstAction`)
          (:`NewEnumerator4`
            (`/Game/TheAtlant_Content/BP/Shark/ScriptedShark/BP_ScriptedShark.CE_StartPath` _linkedscriptedshark))
          (:`NewEnumerator0`
            (`self.M_SwitchToAI` _linkedscriptedshark))
          (:`NewEnumerator2`
            (`self.M_SwitchToAI` _linkedscriptedshark true))))
      (:`else`))))

(fn `UserConstructionScript`)