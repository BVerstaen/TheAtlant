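; BP_ScriptedShark is a shark that follows scripted checkpoints until it is swapped for an AI-driven BP_Shark.
; A Timeline acts as the path tick, turning it toward the current checkpoint and driving FloatingPawnMovement velocity forward.
; A short sphere trace checks for BP_SSHublot obstacles, diverting to an optional bounce checkpoint when BreakCheck fails.
; CE_SwitchToIA spawns the AI shark in place, passes on scale and behavior options, then destroys this actor.
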(event `self.ReceiveBeginPlay`
  ;[1 1 1] SetupBounceCheckPoint
  (bind _bouncecheckpoint (`self.BounceCheckPoint`)
    (:`then`
      (set `/Game/TheAtlant_Content/BP/Shark/ScriptedShark/BP_ScriptedSharkCheckPoint.IsBounceCheckPoint` true _bouncecheckpoint))
    (:`else`)))

(event `CE_SwitchToIA`
  (params (FocusPlayer :type Boolean) (PatrolArea :type "/Game/TheAtlant_Content/BP/Shark/BP_SharkPatrolArea Object Reference") (UpdateParameters :type Boolean) (OptionalParameters :type "/Game/TheAtlant_Content/BP/Shark/ScriptedShark/S_SharkParameters Structure") (NeverForgetPlayer :type Boolean))
  ;[1 1 1] Switch to IA mode
  (bind _returnvalue (`AIBlueprintHelperLibrary.SpawnAIFromClass` "/Game/TheAtlant_Content/BP/Shark/BP_Shark.BP_Shark_C" "/Game/TheAtlant_Content/BP/Shark/IA/BT_Shark.BT_Shark" (`self.K2_GetActorLocation`) (`self.K2_GetActorRotation`) false null))
  (bind _asbp_shark (cast `/Game/TheAtlant_Content/BP/Shark/BP_Shark` _returnvalue)
    (:`then`
      (`/Game/TheAtlant_Content/BP/Shark/BP_SharkPatrolArea.CE_CheckNewShark` PatrolArea)
      (`self.SetActorScale3D` _asbp_shark (`self.GetActorScale3D`))
      (if UpdateParameters
        (`self.UpdateAISharkParameters` OptionalParameters _asbp_shark))
      (if FocusPlayer
        (`/Game/TheAtlant_Content/BP/Shark/BP_Shark.CE_FocusPlayer` _asbp_shark))
      (set `/Game/TheAtlant_Content/BP/Shark/BP_Shark.ForgetPlayer` NeverForgetPlayer _asbp_shark)
      (`self.K2_DestroyActor`))
    (:`CastFailed`
      (`KismetSystemLibrary.PrintString` "Can't spawn Shark" false))))

(event `CE_StartPath`
  (bind _returnvalue (+ (`self.K2_GetActorLocation`) (* (`KismetMathLibrary.GetForwardVector` (`self.K2_GetActorRotation`)) 80.0)))
  ;[1 1 1] Path
  (`Timeline|Timeline` :!label _label
    (:`Update`
      ;;[1 1 1] Rotate to point
      (bind _firstcheckpoint (`self.FirstCheckPoint`)
        (:`then`
          (`self.K2_SetActorRotation` (`KismetMathLibrary.RInterpTo` (`self.K2_GetActorRotation`) (`KismetMathLibrary.FindLookAtRotation` (`self.K2_GetActorLocation`) (`self.K2_GetActorLocation` _firstcheckpoint)) (`GameplayStatics.GetWorldDeltaSeconds`) (`self.RotateSpeed`)))
          ;;[1 1 1] Look if there's a wall in front
          (bind (_outhit _returnvalue_2) (`KismetSystemLibrary.SphereTraceSingleForObjects` _returnvalue _returnvalue 10.0 (`|MakeArray` "ObjectTypeQuery1" "ObjectTypeQuery6" :!type "EObjectTypeQuery Enum")))
          (if _returnvalue_2
            (bind _asbp_sshublot (cast `/Game/TheAtlant_Content/BP/Shark/ScriptedShark/BP_SSHublot` (`.HitActor` (`GameplayStatics.BreakHitResult` _outhit))))
            (bind _isbroken (`/Game/TheAtlant_Content/BP/Shark/ScriptedShark/BP_SSHublot.BreakCheck` _asbp_sshublot))
            (if _isbroken
              ;;[1 1 1] Move to position
              (bind _floatingpawnmovement (`self.FloatingPawnMovement` :!label _label_2)
                (:`then`
                  (set `MovementComponent.Velocity` (* (`self.MoveSpeed`) (`self.GetActorForwardVector`)) _floatingpawnmovement))
                (:`else`))
              (else
                ;;[1 1 1] Bounce to AnotherPoint if possible
                (`self.BounceCheckPoint`
                  (:`then`
                    (`self.K2_SetActorRotation` (* (`self.GetActorForwardVector`) -1.0))
                    ;;;[1 1 1] Setup new bounce point
                    (bind _bouncecheckpoint (`self.BounceCheckPoint`)
                      (:`then`
                        (bind _firstcheckpoint_2 (`self.FirstCheckPoint`)
                          (:`then`
                            (set `/Game/TheAtlant_Content/BP/Shark/ScriptedShark/BP_ScriptedSharkCheckPoint.NextPoint` _firstcheckpoint_2 _bouncecheckpoint)
                            (set `self.FirstCheckPoint` _bouncecheckpoint))
                          (:`else`)))
                      (:`else`)))
                  (:`else`))))
            (else
              (goto _label_2))))
        (:`else`)))))

(event `CE_StopPath`
  ;[1 1 1] Path
  (goto _label :!via `Stop`))

(fn `UpdateAISharkParameters`
  (params (Parameters :type "/Game/TheAtlant_Content/BP/Shark/ScriptedShark/S_SharkParameters Structure") (BP_Shark :type "/Game/TheAtlant_Content/BP/Shark/BP_Shark Object Reference"))
  (bind (_patrolspeed _chasespeed _rotatespeed _wallradius _seeradius _seedistance) (break `/Game/TheAtlant_Content/BP/Shark/ScriptedShark/S_SharkParameters` Parameters))
  (set `/Game/TheAtlant_Content/BP/Shark/BP_Shark.PatrolSpeed` _patrolspeed BP_Shark)
  (set `/Game/TheAtlant_Content/BP/Shark/BP_Shark.ChaseSpeed` _chasespeed BP_Shark)
  (set `/Game/TheAtlant_Content/BP/Shark/BP_Shark.RotateSpeed` _rotatespeed BP_Shark)
  (set `/Game/TheAtlant_Content/BP/Shark/BP_Shark.WallRadius` _wallradius BP_Shark)
  (set `/Game/TheAtlant_Content/BP/Shark/BP_Shark.SeeRadius` _seeradius BP_Shark)
  (set `/Game/TheAtlant_Content/BP/Shark/BP_Shark.SeeDistance` _seedistance BP_Shark))

(fn `UserConstructionScript`)