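; Patrol area actor that assigns itself to sharks inside its collision box and supplies them with movement points.
; On BeginPlay, or when CE_CheckNewShark is called, a box trace over the volume sets each BP_Shark's patrol area reference to this actor.
; GiveRandomPoint scales a random unit vector by the box extent, landing on the inscribed ellipsoid's surface, and GiveRunAwayPoint doubles that offset for fleeing.
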(event `self.ReceiveBeginPlay`
  ;[1 1 1] Check for every shark
  (bind _collision (`self.Collision` :!label _label)
    (:`then`
      (bind _returnvalue (`SceneComponent.K2_GetComponentLocation` _collision))
      (bind _outhits (`KismetSystemLibrary.BoxTraceMultiForObjects` _returnvalue _returnvalue (`BoxComponent.GetScaledBoxExtent` _collision) (`SceneComponent.K2_GetComponentRotation` _collision) (`|MakeArray` "ObjectTypeQuery8" :!type "EObjectTypeQuery Enum")))
      (for _array_element _outhits
        (bind _asbp_shark (cast `/Game/TheAtlant_Content/BP/Shark/BP_Shark` (`.HitActor` (`GameplayStatics.BreakHitResult` _array_element))))
        (set `/Game/TheAtlant_Content/BP/Shark/BP_Shark.BP_PatrolArea` self _asbp_shark)))
    (:`else`)))

(event `CE_CheckNewShark`
  (goto _label))

(fn `GiveRandomPoint`
  (returns (Point :type "Vector Structure"))
  (bind _collision (`self.Collision`)
    (:`then`
      (return (+ (`SceneComponent.K2_GetComponentLocation` _collision) (* (`BoxComponent.GetScaledBoxExtent` _collision) (`KismetMathLibrary.RandomUnitVector`)))))
    (:`else`)))

(fn `GiveRunAwayPoint`
  (returns (Point :type "Vector Structure"))
  (bind _collision (`self.Collision`)
    (:`then`
      (return (+ (`SceneComponent.K2_GetComponentLocation` _collision) (* (`KismetMathLibrary.RandomUnitVector`) (`BoxComponent.GetScaledBoxExtent` _collision) 2.0))))
    (:`else`)))

(fn `UserConstructionScript`)