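; BP_Shark is a shark enemy pawn that kills the player on a hit.
; Hitting the player applies massive damage and tells its AI controller to lose sight of the player.
; Damage taken by the shark is forwarded to the same controller, with a test event to trigger it.
; ChangeSpeed sets the max speed of its FloatingPawnMovement.
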(event `CE_TESTHit`
  ;[1 1 1] Hit
  (`/Game/TheAtlant_Content/BP/Shark/IA/BPI_Damageable.TakeDamage`))

(event `/Game/TheAtlant_Content/BP/Shark/IA/BPI_Damageable.TakeDamage`
  ;[1 1 1] Hit
  (bind _bp_aicontroller (`self.BP_AIController`)
    (:`then`
      (`/Game/TheAtlant_Content/BP/Shark/IA/BP_AISharkController.CE_Hit` _bp_aicontroller))
    (:`else`)))

(event `self.ReceiveHit`
  (params (MyComp :type "PrimitiveComponent Object Reference") (Other :type "Actor Object Reference") (OtherComp :type "PrimitiveComponent Object Reference") (bSelfMoved :type Boolean) (HitLocation :type "Vector Structure") (HitNormal :type "Vector Structure") (NormalImpulse :type "Vector Structure") (Hit :type "HitResult Structure (by ref)"))
  ;[1 1 1] Kill player
  (bind _asbp_player (cast `/Game/TheAtlant_Content/BP/BP_Player` Other))
  (`/Game/TheAtlant_Content/BP/BP_Player.CE_PlayerHit` _asbp_player 999)
  (bind _bp_aicontroller (`self.BP_AIController`)
    (:`then`
      (`/Game/TheAtlant_Content/BP/Shark/IA/BP_AISharkController.CE_LosePlayerSight` _bp_aicontroller))
    (:`else`)))

(fn `ChangeSpeed`
  (params (NewSpeed :type "Float (double-precision)"))
  (bind _floatingpawnmovement (`self.FloatingPawnMovement`)
    (:`then`
      (set `FloatingPawnMovement.MaxSpeed` NewSpeed _floatingpawnmovement))
    (:`else`)))

(fn `UserConstructionScript`)