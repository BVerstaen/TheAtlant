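; BP_gouvernail is a helm object whose lock releases a linked hanging body with a quake effect.
; A harpoon projectile hit on the lock mesh, or an Interact event that also spawns an FS_MasterField, triggers CE_NickFurry.
; That event plays the lock sound and, if the linked body is valid, clears its hanging flag, runs a short-lived shake actor at the player, then destroys the helm after EffectDuration.
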(event `CE_NickFurry`
  ;[1 1 1] Play Quake sound
  (`GameplayStatics.PlaySoundAtLocation` (`self.LockSound`) (`SceneComponent.K2_GetComponentLocation` (`self.GC_BP_LockMesh`)) (struct) 1.0 1.0 0.0 null null null null)
  ;[1 1 1] De-hang body
  (bind _linkedbody (`self.LinkedBody`)
    (:`then`
      (set `/Game/TheAtlant_Content/BP/Item/BP_DeadBody.IsHanging` false _linkedbody)
      ;[1 1 1] Spawn quake effect then destroy
      (bind _returnvalue (`|SpawnActorFromClass` "/Game/TheAtlant_Content/BP/Event_system/EventObjects/BP_EventShakeGouvernail.BP_EventShakeGouvernail_C" (`self.GetTransform` (`GameplayStatics.GetPlayerCharacter` 0)) "Undefined" "MultiplyWithRoot" null null))
      (`/Game/TheAtlant_Content/BP/Event_system/BPI_EventFunctions.CallEvent` _returnvalue)
      (`KismetSystemLibrary.Delay` 1.0)
      (`self.K2_DestroyActor` _returnvalue)
      ;[1 1 1] Timer before destruction
      (`KismetSystemLibrary.K2_SetTimerDelegate` (delegate `CE_Destroy`) (`self.EffectDuration`)))
    (:`else`)))

(event `self.GC_BP_LockMesh.OnComponentHit`
  (params (HitComponent :type "PrimitiveComponent Object Reference") (OtherActor :type "Actor Object Reference") (OtherComp :type "PrimitiveComponent Object Reference") (NormalImpulse :type "Vector Structure") (Hit :type "HitResult Structure (by ref)"))
  (cast `/Game/TheAtlant_Content/BP/BP_HarpoonProjectile` OtherActor)
  (`self.CE_NickFurry`))

(event `CE_Destroy`
  ;[1 1 1] Timer before destruction
  (`self.K2_DestroyActor`))

(event `/Game/TheAtlant_Content/BP/Interaction_System/BPI_InteractableObject.Interact`
  (`|SpawnActorFromClass` "/Engine/EditorResources/FieldNodes/FS_MasterField.FS_MasterField_C" (`self.GetTransform`) "Undefined" "MultiplyWithRoot" null null)
  (`self.CE_NickFurry`))

(fn `UserConstructionScript`
  (`parent.UserConstructionScript`))