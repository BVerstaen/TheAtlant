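; BP_WaterCurrent is a water current volume meant to push the player and objects, with Niagara bubbles whose velocity follows its X scale.
; Each tick, a box trace over its collision rebuilds the list of objects to push.
; Overlap events store and clear the entering actor as the player.
; The timeline that would launch the player and move listed objects is never triggered, so nothing is pushed as wired.
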(event `self.ReceiveTick`
  (params (DeltaSeconds :type "Float (single-precision)"))
  ;[1 1 1] Check for every diodon in water current
  (`KismetArrayLibrary.Array_Clear` (`self.ObjectsToPush`))
  (bind _collision (`self.Collision`)
    (:`then`
      (bind _returnvalue (`SceneComponent.K2_GetComponentLocation` _collision))
      (bind _outhits (`KismetSystemLibrary.BoxTraceMultiForObjects` :`Start` _returnvalue :`End` _returnvalue :`HalfSize` (`BoxComponent.GetScaledBoxExtent` _collision) :`Orientation` (`SceneComponent.K2_GetComponentRotation` _collision) :`ObjectTypes` (`|MakeArray` "ObjectTypeQuery9" :!type "EObjectTypeQuery Enum") :`DrawDebugType` "ForOneFrame"))
      (for _array_element _outhits
        (`KismetArrayLibrary.Array_AddUnique` (`self.ObjectsToPush`) (`.HitActor` (`GameplayStatics.BreakHitResult` _array_element)))))
    (:`else`)))

(event `self.ReceiveBeginPlay`
  (bind _returnvalue_x (`KismetMathLibrary.BreakVector` (`self.GetActorScale3D`)))
  ;[1 1 1] Size particles length by scale
  (bind _ns_watercurrentbubbles (`self.NS_WaterCurrentBubbles`)
    (:`then`
      (`NiagaraComponent.SetVariableVec3` _ns_watercurrentbubbles "InitialVelocity" (`KismetMathLibrary.MakeVector` 0.0 (* _returnvalue_x 250.0))))
    (:`else`)))

(event `self.ReceiveActorBeginOverlap`
  (params (OtherActor :type "Actor Object Reference"))
  ;[1 1 1] get player
  (set `self.PlayerActor` OtherActor))

(event `self.ReceiveActorEndOverlap`
  (params (OtherActor :type "Actor Object Reference"))
  ;[1 1 1] Remove player
  (set `self.PlayerActor` null))

(fn `UserConstructionScript`
  (bind _returnvalue_x (`KismetMathLibrary.BreakVector` (`self.GetActorScale3D`)))
  (bind _ns_watercurrentbubbles (`self.NS_WaterCurrentBubbles`)
    (:`then`
      (`NiagaraComponent.SetNiagaraVariableVec3` _ns_watercurrentbubbles "InitialVelocity" (`KismetMathLibrary.MakeVector` 0.0 (* _returnvalue_x 250.0))))
    (:`else`)))