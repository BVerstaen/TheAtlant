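; BP_Cage is the cage that receives dead bodies and handles the victory cinematic.
; Interacting with an objective body reports the found corpse to GI_TheAtlant and destroys the body, while a possessed one only prints a debug message.
; On BeginPlay it registers with the game instance's launch-victory dispatcher.
; When that fires, it plays VictoryCine, waits for the sequence length, then calls the game instance's win event.
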(event `self.ReceiveBeginPlay`
  ;[1 1 1] Get the game instance
  (bind _asgi_the_atlant (cast `/Game/TheAtlant_Content/BP/Game/GI_TheAtlant` (`GameplayStatics.GetGameInstance`)))
  (bind _output_get (set `self.GI_TheAtlant` _asgi_the_atlant))
  (add `/Game/TheAtlant_Content/BP/Game/GI_TheAtlant.ED_OnLaunchVictory` _output_get (delegate `CE_LaunchVictory`)))

(event `CE_LaunchVictory`
  ;[1 1 1] Get the game instance
  (bind _victorycine (`self.VictoryCine`)
    (:`then`
      (bind _sequenceplayer (`LevelSequenceActor.SequencePlayer` _victorycine)
        (:`then`
          ;[1 1 1] Wait until sequence ends
          (`MovieSceneSequencePlayer.Play` _sequenceplayer)
          (`KismetSystemLibrary.Delay` (`TimeManagementBlueprintLibrary.Conv_QualifiedFrameTimeToSeconds` (`MovieSceneSequencePlayer.GetEndTime` _sequenceplayer)))
          ;[1 1 1] Launch end game
          (bind _gi_theatlant (`self.GI_TheAtlant`)
            (:`then`
              (`/Game/TheAtlant_Content/BP/Game/GI_TheAtlant.ED_OnWinGame` _gi_theatlant))
            (:`else`)))
        (:`else`)))
    (:`else`)))

(event `/Game/TheAtlant_Content/BP/Interaction_System/BPI_InteractableObject.InteractWithItem`
  (params (Item :type "/Game/TheAtlant_Content/BP/BP_ParentItem Object Reference"))
  ;[1 1 1] If put a dead body, then destroy actor & decrease corpse
  (if (`/Game/TheAtlant_Content/BP/BP_ParentItem.IsDeadBody` Item)
    (bind _asbp_dead_body (cast `/Game/TheAtlant_Content/BP/Item/BP_DeadBody` Item))
    (switch `/Game/TheAtlant_Content/Data/Enum/E_DeadBodyTypes` (`/Game/TheAtlant_Content/BP/Item/BP_DeadBody.Type` _asbp_dead_body)
      (:`NewEnumerator0`
        (bind _gi_theatlant (`self.GI_TheAtlant`)
          (:`then`
            (`/Game/TheAtlant_Content/BP/Game/GI_TheAtlant.CE_FoundCorpse` _gi_theatlant true)
            (`self.K2_DestroyActor` Item))
          (:`else`)))
      (:`NewEnumerator2`
        (`KismetSystemLibrary.PrintString` "WTF, how did you... OK" false)))))

(fn `UserConstructionScript`)