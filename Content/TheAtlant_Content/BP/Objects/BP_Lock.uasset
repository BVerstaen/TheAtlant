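; BP_Lock is a lock that a harpoon shot triggers to signal its linked BP_InteractDoor.
; On BeginPlay it searches all interact doors for a matching ID and stores that reference.
; A BP_HarpoonProjectile hit on the lock mesh plays a sound and calls CE_Interact, which calls LeverPulled on the linked door once.
; The lock then destroys itself after an effect delay.
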(event `self.ReceiveBeginPlay`
  ;[1 0.4348 0.8352] Link lever to correct door
  (bind _outactors (`GameplayStatics.GetAllActorsOfClass` "/Game/TheAtlant_Content/BP/Interaction_System/Interactable_Objects/BP_InteractDoor.BP_InteractDoor_C"))
  (bind _returnvalue (`KismetArrayLibrary.Array_Length` _outactors))
  (if (> _returnvalue 0)
    (for _index (range _returnvalue)
      (bind _output (`|GetArrayItem` _outactors _index))
      (bind _id (`/Game/TheAtlant_Content/BP/Interaction_System/Interactable_Objects/BP_InteractDoor.getID` _output))
      (if (== _id (`self.Id`))
        (set `self.DoorRef` _output)
        (set `self.IsLinked` true)
        (`KismetSystemLibrary.PrintString` "Linked to correct door" false)
        (break)))))

(event `CE_Interact`
  ;[0.3903 0.8525 1] Interact
  (if (`self.IsLinked`)
    (if true
      (if (not (`self.Used`))
        (set `self.Used` true :!label _label)
        (bind _doorref (`self.DoorRef`)
          (:`then`
            (`/Game/TheAtlant_Content/BP/Interaction_System/Interactable_Objects/BP_InteractDoor.LeverPulled` _doorref))
          (:`else`)))
      (else
        (goto _label)))))

(event `self.GC_BP_LockMesh.OnComponentHit`
  (params (HitComponent :type "PrimitiveComponent Object Reference") (OtherActor :type "Actor Object Reference") (OtherComp :type "PrimitiveComponent Object Reference") (NormalImpulse :type "Vector Structure") (Hit :type "HitResult Structure (by ref)"))
  ;[0.3903 0.8525 1] Interact
  ;;[1 1 1] If hit by harpoon
  (cast `/Game/TheAtlant_Content/BP/BP_HarpoonProjectile` OtherActor)
  (`GameplayStatics.PlaySoundAtLocation` (`self.LockSound`) (`SceneComponent.K2_GetComponentLocation` (`self.GC_BP_LockMesh`)) (struct) 1.0 1.0 0.0 null null null null)
  (`self.CE_Interact`)
  ;;[1 1 1] Destroy self
  (`KismetSystemLibrary.Delay` (`self.EffectDuration`))
  (`self.K2_DestroyActor`))

(fn `UserConstructionScript`)