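; Interactable trap door that switches a water current on and off, toggled through Interact or DragEvent.
; A timeline swings the hatch, ignoring input while moving, then spawns BP_WaterCurrent after opening (if enabled) or destroys it after closing.
; An editor preview current follows a configurable transform; BeginPlay removes it and moves the spawn point there.
; The spawned current is destroyed when the trap is removed from the world.
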(event `self.ReceiveBeginPlay`
  ;[1 1 1] Set default rotation
  ;;[1 1 1] Remove preview Current
  (bind _bp_watercurrent (`self.BP_WaterCurrent`)
    (:`then`
      (`ActorComponent.K2_DestroyComponent` _bp_watercurrent)
      ;;[1 1 1] Set Point
      (bind _watercurrentspawnpoint (`self.WaterCurrentSpawnPoint`)
        (:`then`
          (`SceneComponent.K2_SetRelativeTransform` _watercurrentspawnpoint (`self.WaterCurrentTransform`) false false))
        (:`else`)))
    (:`else`)))

(event `self.ReceiveEndPlay`
  (params (EndPlayReason :type "EEndPlayReason Enum" :default "Destroyed"))
  ;[1 1 1] Destroy Water Current
  (switch `EEndPlayReason` EndPlayReason
    (:`RemovedFromWorld`
      (bind _watercurrentactor (`self.WaterCurrentActor`)
        (:`then`
          (`self.K2_DestroyActor` _watercurrentactor))
        (:`else`)))))

(event `CE_Interact`
  ;[1 1 1] Interaction
  (if (not (`self.IsBusy`))
    (bind _output_get (set `self.IsOpened` (not (`self.IsOpened`))))
    (if _output_get
      (set `self.IsBusy` true)
      ;[1 1 1] Rotation Animation
      (bind (_direction _rotationlerp) (`Timeline|tl_TrapDoorAnimation` :!label _label)
        (:`Update`
          (bind _hauttrapposition (`self.HautTrapPosition`)
            (:`then`
              (`SceneComponent.K2_SetRelativeRotation` _hauttrapposition (`KismetMathLibrary.MakeRotator` 0.0 0.0 (`KismetMathLibrary.Lerp` 0.0 -90.0 _rotationlerp)) false false))
            (:`else`)))
        (:`Finished`
          ;;[1 1 1] Create / destroy the water current
          (set `self.IsBusy` false)
          (switch `ETimelineDirection` _direction
            (:`Forward`
              (if (`self.SpawnWaterCurrent`)
                (`self.CE_CreateWaterCurrent`)))
            (:`Backward`
              (`self.CE_DestroyWaterCurrent`)))))
      (else
        (set `self.IsBusy` true)
        (goto _label :!via `Reverse`)))))

(event `/Game/TheAtlant_Content/BP/Interaction_System/BPI_InteractableObject.Interact`
  ;[1 1 1] Interaction
  (`self.CE_Interact`))

(event `CE_CreateWaterCurrent`
  ;[1 1 1] Create / Destroy the water current
  (`self.WaterCurrentActor`
    (:`then`)
    (:`else`
      (bind _watercurrentspawnpoint (`self.WaterCurrentSpawnPoint`)
        (:`then`
          (bind _returnvalue (`|SpawnActorFromClass` "/Game/TheAtlant_Content/BP/Objects/BP_WaterCurrent.BP_WaterCurrent_C" (`SceneComponent.K2_GetComponentToWorld` _watercurrentspawnpoint) "Undefined" "MultiplyWithRoot" null null))
          (set `self.WaterCurrentActor` _returnvalue))
        (:`else`)))))

(event `CE_DestroyWaterCurrent`
  ;[1 1 1] Create / Destroy the water current
  (bind _watercurrentactor (`self.WaterCurrentActor`)
    (:`then`
      (`self.K2_DestroyActor` _watercurrentactor))
    (:`else`)))

(fn `DragEvent`
  (params (ActivateEvent :type Boolean))
  (returns (ShouldUnhook :type Boolean))
  (if ActivateEvent
    (`self.CE_Interact`))
  (return true))

(fn `UserConstructionScript`
  (bind _bp_watercurrent (`self.BP_WaterCurrent`)
    (:`then`
      (`SceneComponent.K2_SetRelativeTransform` _bp_watercurrent (`self.WaterCurrentTransform`) false false))
    (:`else`)))