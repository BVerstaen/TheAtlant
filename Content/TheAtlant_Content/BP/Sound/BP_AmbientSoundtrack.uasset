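; BP_AmbientSoundtrack controls the ambient music, switching between two tracks and linking them to player stress.
; Switch events fire trigger parameters on its Audio component, with CurrentMusic preventing a restart of the track already selected.
; Switching to track 1 calls the player's stress decrement event, and track 2 calls the increment.
; BeginPlay and StartOver request track 1, while Stop halts the audio.
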(event `self.ReceiveBeginPlay`
  ;[1 1 1] Maybe make it so that it starts when you respawn and not on begin play
  (`self.SwitchTo1` :!label _label))

(event `Stop`
  (`AudioComponent.Stop` (`self.Audio`)))

(event `StartOver`
  ;[1 1 1] Maybe make it so that it starts when you respawn and not on begin play
  (goto _label))

(event `SwitchTo1`
  ;[1 1 1] Switches
  (if (!= (`self.CurrentMusic`) 1)
    (`AudioParameterControllerInterface.SetTriggerParameter` (`self.Audio`) "Audio1")
    (set `self.CurrentMusic` 1)
    (bind _asbp_player (cast `/Game/TheAtlant_Content/BP/BP_Player` (`GameplayStatics.GetPlayerPawn` 0)))
    (`/Game/TheAtlant_Content/BP/BP_Player.CE_DecrementStress` _asbp_player)))

(event `SwitchTo2`
  ;[1 1 1] Switches
  (if (!= (`self.CurrentMusic`) 2)
    (`AudioParameterControllerInterface.SetTriggerParameter` (`self.Audio`) "Audio2")
    (set `self.CurrentMusic` 2)
    (bind _asbp_player (cast `/Game/TheAtlant_Content/BP/BP_Player` (`GameplayStatics.GetPlayerPawn` 0)))
    (`/Game/TheAtlant_Content/BP/BP_Player.CE_IncrementStress` _asbp_player)))

(fn `UserConstructionScript`)