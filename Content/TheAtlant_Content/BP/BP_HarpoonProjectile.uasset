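; Roped harpoon projectile fired by the player, used to drag, grip, break or damage what it hits.
; On hit it attaches or notifies draggables, flags grippable surfaces, fractures geometry collections via a spawned field, or damages targets.
; Pulling and unhooking use physics forces toward the player, while Tick unhooks and clamps it beyond maximum rope length.
; It self-destructs on player death, player or harpoon contact, or a timer started by unhooking.
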(event `CE_Initialize`
  ;[1 1 1] Set End of rope
  (bind _bp_player (`self.BP_Player`)
    (:`then`
      (add `/Game/TheAtlant_Content/BP/BP_Player.ED_OnPlayerDied` _bp_player (delegate `CE_Destroy Harpoon`))
      (bind _ropeplayerpoint (`/Game/TheAtlant_Content/BP/BP_Player.RopePlayerPoint` _bp_player)
        (:`then`
          (bind _rope (`self.Rope`)
            (:`then`
              (`CableComponent.SetAttachEndToComponent` _rope _ropeplayerpoint "None"))
            (:`else`)))
        (:`else`)))
    (:`else`)))

(event `CE_PullObject`
  ;[1 1 1] Pull object towards player (or activate pull event)
  ;;[1 1 1] Activate event & unhook harpoon
  (bind _attachedobject (`self.AttachedObject`)
    (:`then`
      (bind _shouldunhook (message `/Game/TheAtlant_Content/Interfaces/BPI_Draggable.DragEvent` _attachedobject true))
      (if _shouldunhook
        (`self.CE_UnHook` true)
        (else
          ;;[1 1 1] Else physics pull
          (bind _collision (`self.Collision`)
            (:`then`
              (`PrimitiveComponent.SetSimulatePhysics` _collision true)
              (`PrimitiveComponent.AddForce` _collision (* (* (`self.PullObjectForce`) -1.0) (`KismetMathLibrary.Normal` (- (`self.K2_GetActorLocation`) (`self.K2_GetActorLocation` (`GameplayStatics.GetPlayerCharacter` 0))))) "None" false))
            (:`else`)))))
    (:`else`)))

(event `CE_Destroy Harpoon`
  ;[1 1 1] Destroy Harpoon if player died
  (`AudioComponent.Stop` (`self.HarpoonNoises`))
  (`self.K2_DestroyActor`))

(event `CE_UnHook`
  (params (ShouldAddForce :type Boolean))
  ;[1 1 1] Unhook & drag to player
  (if (not (`self.HasAutoDestructTimerLaunched`))
    (`KismetSystemLibrary.K2_SetTimerDelegate` (delegate `CE_AutoDestroyHarpoon`) (`self.TimeBeforeAutoDestroy`))
    (set `self.HasAutoDestructTimerLaunched` true))
  (`self.ReloadSound`)
  (set `self.IsAggripable` false)
  (`self.CE_ChangeCollisionProfile`)
  ;;[1 1 1] Detach attached actor
  (bind _attachedobject (`self.AttachedObject`)
    (:`then`
      (`self.K2_DetachFromActor` _attachedobject "KeepWorld" "KeepWorld" "KeepWorld"))
    (:`else`
      _))
  (set `self.AttachedObject` null)
  ;;[1 1 1] Destroy Projectile component & add force to player
  (bind _projectilemovement (`self.ProjectileMovement`)
    (:`then`
      (`ActorComponent.K2_DestroyComponent` _projectilemovement))
    (:`else`
      _))
  (if ShouldAddForce
    (bind _collision (`self.Collision`)
      (:`then`
        (`PrimitiveComponent.SetSimulatePhysics` _collision true)
        (`PrimitiveComponent.AddForce` _collision (* (* (`self.RetraceForce`) -1.0) (`KismetMathLibrary.Normal` (- (`self.K2_GetActorLocation`) (`self.K2_GetActorLocation` (`GameplayStatics.GetPlayerCharacter` 0))))) "None" true)
        (`self.ReloadSound`))
      (:`else`))))

(event `CE_AutoDestroyHarpoon`
  ;[1 1 1] Unhook & drag to player
  (`KismetSystemLibrary.PrintString` "Destroy harpoon" false)
  (`self.DestroyHarpoon`))

(event `self.ReceiveTick`
  (params (DeltaSeconds :type "Float (single-precision)"))
  ;[1 1 1] Unhook the harpoon if too far away
  (if (> (`KismetMathLibrary.Vector_Distance` (`self.K2_GetActorLocation` (`GameplayStatics.GetPlayerCharacter` 0)) (`self.K2_GetActorLocation`)) (`self.MaxLength`))
    (`self.CE_UnHook` false)
    ;;[1 1 1] Reset Velocity
    (bind _collision (`self.Collision`)
      (:`then`
        (`PrimitiveComponent.SetPhysicsLinearVelocity` _collision (0.0 0.0 0.0) false "None")
        (bind _bp_player (`self.BP_Player`)
          (:`then`
            (`self.K2_SetActorLocation` (+ (* (- (`self.K2_GetActorLocation`) (`self.K2_GetActorLocation` _bp_player)) 0.99) (`self.K2_GetActorLocation` _bp_player)))
            (`self.Reload Stop`))
          (:`else`)))
      (:`else`))))

(event `CE_ChangeCollisionProfile`
  ;[1 1 1] Change collision
  (bind _collision (`self.Collision`)
    (:`then`
      (`PrimitiveComponent.SetCollisionObjectType` _collision "ECC_GameTraceChannel5")
      (bind _mesh (`self.Mesh`)
        (:`then`
          (`PrimitiveComponent.SetCollisionObjectType` _mesh "ECC_GameTraceChannel5"))
        (:`else`)))
    (:`else`)))

(event `self.ReceiveHit`
  (params (MyComp :type "PrimitiveComponent Object Reference") (Other :type "Actor Object Reference") (OtherComp :type "PrimitiveComponent Object Reference") (bSelfMoved :type Boolean) (HitLocation :type "Vector Structure") (HitNormal :type "Vector Structure") (NormalImpulse :type "Vector Structure") (Hit :type "HitResult Structure (by ref)"))
  (bind (_bblockinghit _binitialoverlap _time _distance _location _impactpoint _normal _impactnormal _physmat _hitactor _hitcomponent) (`GameplayStatics.BreakHitResult` Hit))
  ;[1 1 1] Hit Event
  (`self.Hit`)
  ;;[1 1 1] Remove projectile component (if possible)
  (bind _projectilemovement (`self.ProjectileMovement`)
    (:`then`
      (`ActorComponent.K2_DestroyComponent` _projectilemovement))
    (:`else`
      _))
  ;;[1 1 1] If hit by player -> delete projectile
  (cast `/Game/TheAtlant_Content/BP/BP_Player` _hitactor
    (:`then`
      (`self.DestroyHarpoon` :!label _label))
    (:`CastFailed`
      (cast `/Game/TheAtlant_Content/BP/BP_HarpoonProjectile` _hitactor
        (:`then`
          (goto _label))
        (:`CastFailed`
          ;;[1 1 1] Else check if is an draggable objet
          (if (`KismetSystemLibrary.DoesImplementInterface` _hitactor "/Game/TheAtlant_Content/Interfaces/BPI_Draggable.BPI_Draggable_C")
            ;;;[1 1 1] Reset Velocity
            (bind _collision (`self.Collision`)
              (:`then`
                (`PrimitiveComponent.SetPhysicsLinearVelocity` _collision (0.0 0.0 0.0) false "None")
                (bind _bp_player (`self.BP_Player`)
                  (:`then`
                    (set `/Game/TheAtlant_Content/BP/BP_Player.CanDrag` true _bp_player)
                    (bind _output_get (set `self.AttachedObject` _hitactor))
                    (bind _shouldunhook (message `/Game/TheAtlant_Content/Interfaces/BPI_Draggable.DragEvent` _output_get false))
                    (if (not _shouldunhook)
                      (bind _tip (`self.Tip`)
                        (:`then`
                          (`self.K2_AttachToComponent` _output_get _tip "None" "SnapToTarget" "KeepWorld" "SnapToTarget" true))
                        (:`else`))))
                  (:`else`)))
              (:`else`))
            (else
              ;;[1 1 1] Else check if can pull player
              (if (`KismetSystemLibrary.DoesImplementInterface` _hitactor "/Game/TheAtlant_Content/Interfaces/BPI_Aggripable.BPI_Aggripable_C")
                (set `self.IsAggripable` true)
                (else
                  ;;[1 1 1] Else Check if should destroy
                  (cast `GeometryCollectionActor` _hitactor
                    (:`then`
                      (bind _returnvalue (`|SpawnActorFromClass` "/Engine/EditorResources/FieldNodes/FS_MasterField.FS_MasterField_C" (`KismetMathLibrary.MakeTransform` (`self.K2_GetActorLocation`)) "Undefined" "MultiplyWithRoot" null null :!label _label_2))
                      (set `/Engine/EditorResources/FieldNodes/FS_MasterField.ActivationType` "NewEnumerator4" _returnvalue)
                      (`/Engine/EditorResources/FieldNodes/FS_MasterField.CE_Trigger` _returnvalue)
                      (`self.K2_DestroyActor` _returnvalue)
                      (`self.CE_UnHook` false))
                    (:`CastFailed`
                      ;;;[1 1 1] Look if geometry is inside a BP
                      (cast `GeometryCollectionComponent` _hitcomponent
                        (:`then`
                          (goto _label_2))
                        (:`CastFailed`
                          ;;[1 1 1] Else Check if should give damage
                          (if (`KismetSystemLibrary.DoesImplementInterface` _hitactor "/Game/TheAtlant_Content/BP/Shark/IA/BPI_Damageable.BPI_Damageable_C")
                            (message `/Game/TheAtlant_Content/BP/Shark/IA/BPI_Damageable.TakeDamage` _hitactor)
                            (`self.CE_UnHook` false)))))))))))))))

(event `ReloadSound`
  ;[1 0.4584 0.8271] Sound triggers
  (if (not (`self.isReloadSoundPlaying`))
    (`AudioParameterControllerInterface.SetTriggerParameter` (`self.HarpoonNoises`) "Reload")
    (set `self.isReloadSoundPlaying` true)))

(event `Reload Stop`
  ;[1 0.4584 0.8271] Sound triggers
  (`AudioParameterControllerInterface.SetTriggerParameter` (`self.HarpoonNoises`) "ReloadStop")
  (set `self.isReloadSoundPlaying` false))

(event `Hit`
  ;[1 0.4584 0.8271] Sound triggers
  (`AudioParameterControllerInterface.SetTriggerParameter` (`self.HarpoonNoises`) "Hit"))

(fn `DestroyHarpoon`
  (bind _bp_player (`self.BP_Player`)
    (:`then`
      (set `/Game/TheAtlant_Content/BP/BP_Player.CanDrag` false _bp_player)
      (`/Game/TheAtlant_Content/BP/BP_Player.CE_ShowHarpoonTip` _bp_player true)
      (`/Game/TheAtlant_Content/BP/BP_Player.CE_StopAnim` _bp_player)
      (`self.Reload Stop`)
      (`self.K2_DestroyActor`))
    (:`else`)))

(fn `UserConstructionScript`)