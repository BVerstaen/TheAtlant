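; Player pawn for TheAtlant, an underwater diver with a helmet lamp, harpoon, breathing audio and radio.
; Damage swaps the suit's glass material and starts leak particles; death removes input, tilts the camera, notifies listeners and drops any carried object.
; Timelines drive harpoon draw/hide, FOV and death camera, while a random-interval timer flickers the spotlight.
; Jumpscares snap the shark to an attach point and flag its blackboard; construction stores the respawn transform.
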(event `StartCalmAmbience`
  ;[1 0.02537 0.9309] Ambient Start
  (bind _asgi_the_atlant (cast `/Game/TheAtlant_Content/BP/Game/GI_TheAtlant` (`GameplayStatics.GetGameInstance`)))
  (`/Game/TheAtlant_Content/BP/Game/GI_TheAtlant.StartMusic` _asgi_the_atlant)
  (`AudioComponent.Play` (`self.Breathing`) 0.0)
  (`self.CE_DecrementStress`))

(event `CE_IncrementStress`
  ;[1 0.3316 0.9699] Breathing
  (if (not (`self.Is Breathing Hard`))
    (`AudioParameterControllerInterface.SetTriggerParameter` (`self.Breathing`) "Audio2")
    (`KismetSystemLibrary.PrintString` "Audio2")
    (set `self.Is Breathing Hard` true)))

(event `self.ReceiveBeginPlay`
  ;[1 1 1] Get default spotlight intensity
  (bind _spotlight (`self.SpotLight`)
    (:`then`
      (set `self.DefaultSpotLightIntensity` (`LightComponentBase.Intensity` _spotlight))
      ;[1 1 1] Get default harpoon transform
      (bind _harpoonmesh (`self.HarpoonMesh`)
        (:`then`
          (set `self.HarpoonDefaultTransform` (`SceneComponent.GetRelativeTransform` _harpoonmesh))
          ;[1 1 1] Randomly flickers the spotlight
          (`KismetSystemLibrary.K2_SetTimerDelegate` (delegate `CE_FlickerLight`) (`KismetMathLibrary.RandomFloatInRange` 5.0 10.0) true)
          (`self.StartCalmAmbience`))
        (:`else`)))
    (:`else`)))

(event `CE_DecrementStress`
  ;[1 0.3316 0.9699] Breathing
  (if (`self.Is Breathing Hard`)
    (`AudioParameterControllerInterface.SetTriggerParameter` (`self.Breathing`) "Audio1")
    (`KismetSystemLibrary.PrintString` "Audio1")
    (set `self.Is Breathing Hard` false)))

(event `BreathingParticles`
  ;[0.5455 1 0.4422] Breathing Particles
  (`/Engine/EditorBlueprintResources/StandardMacros.DecrementInt` (`self.BreathingCounter`)
    (:`  `
      (if (`self.IsInQTE`)
        _
        (elif (> (`self.HealthPoints`) 0)
          (if (<= (`self.BreathingCounter`) 0)
            (`ActorComponent.Activate` (`self.BreathingBubbles`) false)
            (`GameplayStatics.PlaySoundAtLocation` "/Game/TheAtlant_Content/Audio/Player/BubbleOut.BubbleOut" (`SceneComponent.K2_GetComponentLocation` (`self.BreathingBubbles`)) (struct) 1.0 1.0 0.0 null null null null)
            (set `self.BreathingCounter` 3)))))))

(event `CE_FlickerLight`
  ;[1 1 1] Randomly flickers the spotlight
  (bind _spotlight (`self.SpotLight`)
    (:`then`
      (`LightComponent.SetIntensity` _spotlight (* (`self.DefaultSpotLightIntensity`) (`KismetMathLibrary.RandomFloatInRange` 0.1 0.7)))
      (`KismetSystemLibrary.Delay` (`KismetMathLibrary.RandomFloatInRange` 0.0 0.0))
      (`LightComponent.SetIntensity` _spotlight (`self.DefaultSpotLightIntensity`)))
    (:`else`)))

(event `CE_PlayerHit`
  (params (Damage :type Integer))
  (bind _healthpoints (`self.HealthPoints`))
  ;[1 1 1] Hit & Death
  ;;[1 1 1] Look if player not already dead
  (if (> (`self.HealthPoints`) 0)
    ;;[1 1 1] Guard
    (if (> Damage 0)
      ;;[1 1 1] Hit
      (`self.PlayerHurtSound`)
      (set `self.HealthPoints` (- (`self.HealthPoints`) Damage))
      (`self.CE_UpdateScaphandreMesh`)
      ;;[1 0 0.7016] Particle Activate
      (if (== (`self.HealthPoints`) 4)
        (`ActorComponent.Activate` (`self.WaterParticles`) false))
      (if (== (`self.HealthPoints`) 2)
        (`ActorComponent.Activate` (`self.WaterParticles1`) false))
      ;;[1 1 1] Death & remove controls
      (if (<= _healthpoints 0)
        (`EnhancedInputSubsystemInterface.RemoveMappingContext` (pcsubsystem `EnhancedInputLocalPlayerSubsystem` (`GameplayStatics.GetPlayerController` 0)) "/Game/TheAtlant_Content/Input/IMC_Gameplay.IMC_Gameplay" (struct))
        (`self.PlayerDeathSound`)
        (bind _aspc_the_atlant (cast `/Game/TheAtlant_Content/BP/Game/PC_TheAtlant` (`GameplayStatics.GetPlayerController` 0)))
        ;;[1 1 1] Death animation
        (`/Game/TheAtlant_Content/BP/Game/PC_TheAtlant.CE_HardStopMoveAnimation` _aspc_the_atlant)
        (bind (_direction _camlerp) (`Timeline|tl_DeathAnimation` :!via `PlayFromStart`)
          (:`Update`
            (bind _camera (`self.Camera`)
              (:`then`
                (set `CameraComponent.bUsePawnControlRotation` false _camera)
                (bind (_relativelocation_x _relativelocation_y) (`KismetMathLibrary.BreakVector` (`SceneComponent.RelativeLocation` _camera)))
                (`SceneComponent.K2_SetRelativeLocation` _camera (`KismetMathLibrary.MakeVector` _relativelocation_x _relativelocation_y (`KismetMathLibrary.Lerp` 50.0 0.0 _camlerp)) false false)
                (`SceneComponent.K2_SetRelativeRotation` _camera (`KismetMathLibrary.MakeRotator` (`KismetMathLibrary.Lerp` 0.0 15.0 _camlerp)) false false))
              (:`else`)))
          (:`Finished`
            ;;[0.9435 1 0.96] Force drop, Event Everyone & Destroy
            (`self.ED_OnPlayerDied`)
            (bind _carriedobject (`self.CarriedObject`)
              (:`then`
                (`/Game/TheAtlant_Content/BP/BP_ParentItem.CE_Drop` _carriedobject self (`self.K2_GetActorLocation`)))
              (:`else`))))
        (else
          (`self.ED_OnPlayerHit` _healthpoints)))
      (else
        (`KismetSystemLibrary.PrintString` "Damage can't be negative" false)))))

(event `PlayerHurtSound`
  ;[1 0.233 0.9786] PlayerSound
  (bind _returnvalue (`GameplayStatics.SpawnSoundAtLocation` "/Game/TheAtlant_Content/Audio/_MetaSounds/Player/MS_Player.MS_Player" (`SceneComponent.K2_GetComponentLocation` (`self.Mesh`)) (struct) 1.0 1.0 0.0 null null))
  (`AudioParameterControllerInterface.SetTriggerParameter` _returnvalue "Hurt"))

(event `CE_TESTDeath`
  ;[1 1 1] Hit & Death
  (`self.CE_PlayerHit` 5))

(event `PlayerDeathSound`
  ;[1 0.233 0.9786] PlayerSound
  (bind _returnvalue (`GameplayStatics.SpawnSoundAtLocation` "/Game/TheAtlant_Content/Audio/_MetaSounds/Player/MS_Player.MS_Player" (`SceneComponent.K2_GetComponentLocation` (`self.Mesh`)) (struct) 1.0 1.0 0.0 null null))
  (`AudioParameterControllerInterface.SetTriggerParameter` _returnvalue "Death")
  (if (`KismetSystemLibrary.IsValid` (stale `PlayerHurtSound` _returnvalue))
    (`AudioComponent.Stop` (stale `PlayerHurtSound` _returnvalue))))

(event `CE_UpdateScaphandreMesh`
  ;[1 1 1] Hit & Death
  ;;[1 1 1] Update mesh
  (bind _scafendre (`self.Scafendre`)
    (:`then`
      (`PrimitiveComponent.SetMaterial` _scafendre 1 (`|GetArrayItem` (`self.ScaphandreVitreMaterial`) (`KismetMathLibrary.Clamp` (`self.HealthPoints`) 0 5))))
    (:`else`)))

(event `CE_PlayHarpoonHide`
  (params (delay :type "Float (double-precision)"))
  (bind (_harpoondefaulttransform_location _harpoondefaulttransform_rotation) (`KismetMathLibrary.BreakTransform` (`self.HarpoonDefaultTransform`)))
  ;[1 1 1] Play Harpoon animation
  (`KismetSystemLibrary.Delay` delay)
  (bind (_direction _animationlerp) (`Timeline|tl_DrawHarpoon` :!label _label)
    (:`Update`
      (bind _harpoonmesh (`self.HarpoonMesh`)
        (:`then`
          (`SceneComponent.K2_SetRelativeLocation` _harpoonmesh (`KismetMathLibrary.VLerp` _harpoondefaulttransform_location (- _harpoondefaulttransform_location (85.0 0.0 0.0)) _animationlerp) false false)
          (`SceneComponent.K2_SetRelativeRotation` _harpoonmesh (`KismetMathLibrary.RLerp` _harpoondefaulttransform_rotation (struct :`Yaw` -90.0 :`Roll` 70.0) _animationlerp true) false false))
        (:`else`)))))

(event `CE_GetJumpscared`
  (params (Shark :type "/Game/TheAtlant_Content/BP/Shark/BP_Shark Object Reference"))
  ;[1 0.9123 0.4425] Jumpscared
  (bind _asbp_aishark_controller (cast `/Game/TheAtlant_Content/BP/Shark/IA/BP_AISharkController` (`AIBlueprintHelperLibrary.GetAIController` Shark)))
  (bind _blackboard (`AIController.Blackboard` _asbp_aishark_controller)
    (:`then`
      (`BlackboardComponent.SetValueAsBool` _blackboard "IsPlayerDead" true)
      (`SceneComponent.K2_SetWorldLocation` (`Actor.RootComponent` Shark) (`SceneComponent.K2_GetComponentLocation` (`self.SharkJumpscarePoint`)) false false)
      (`self.K2_SetActorRotation` Shark (`SceneComponent.K2_GetComponentRotation` (`self.SharkJumpscarePoint`)) false))
    (:`else`)))

(event `CE_ShowHarpoonTip`
  (params (Show :type Boolean))
  ;[1 1 1] Harpoon animations
  ;;[1 1 1] Show tip
  (bind _harpoontip (`self.HarpoonTip`)
    (:`then`
      (`SceneComponent.SetVisibility` _harpoontip Show false))
    (:`else`)))

(event `CE_PlayWalkAnimation`
  (params (IsWalking :type Boolean))
  ;[1 1 1] Harpoon animations
  ;;[1 1 1] Walk
  (if IsWalking
    (bind _harpoonmesh (`self.HarpoonMesh`)
      (:`then`
        (`SkeletalMeshComponent.PlayAnimation` _harpoonmesh "/Game/TheAtlant_Content/GA/Harpon/Animations/harpon_walk.harpon_walk" true)
        (bind _harpoontip (`self.HarpoonTip`)
          (:`then`
            (`SceneComponent.K2_SetRelativeLocation` _harpoontip (-58.0 -136.0 -14.0) false false))
          (:`else`)))
      (:`else`))
    (else
      (`SkeletalMeshComponent.Stop` _harpoonmesh))))

(event `CE_PlayHarpoonDraw`
  (params (delay :type "Float (double-precision)"))
  ;[1 1 1] Play Harpoon animation
  (`KismetSystemLibrary.Delay` delay)
  (`self.CarriedObject`
    (:`then`)
    (:`else`
      (goto _label :!via `Reverse`))))

(event `CE_PlayReloadAnim`
  (params (CheckDrag :type Boolean))
  ;[1 1 1] Harpoon animations
  ;;[1 1 1] Reload
  (if (or (not CheckDrag) (and CheckDrag (`self.CanDrag`)))
    (bind _harpoonmesh (`self.HarpoonMesh`)
      (:`then`
        (if (not (`SkeletalMeshComponent.IsPlaying` _harpoonmesh))
          (`SkeletalMeshComponent.PlayAnimation` _harpoonmesh "/Game/TheAtlant_Content/GA/Harpon/Animations/harpon_reload.harpon_reload" false)))
      (:`else`))))

(event `CE_FOVAnimationActivate`
  ;[1 1 1] Change cam FOV
  (bind (_direction _camlerp) (`Timeline|tl_ChangeFOV` :!label _label_2)
    (:`Update`
      (bind _camera (`self.Camera`)
        (:`then`
          (`CameraComponent.SetFieldOfView` _camera (`KismetMathLibrary.Lerp` 90.0 115.0 _camlerp)))
        (:`else`)))))

(event `CE_FOVAnimationDeActivate`
  ;[1 1 1] Change cam FOV
  (goto _label_2 :!via `Reverse`))

(event `CE_StopAnim`
  ;[1 1 1] Harpoon animations
  ;;[1 1 1] Reload
  ;;;[1 1 1] Play walk anim to reset position
  (bind _arms (`self.Arms`)
    (:`then`
      (`SkeletalMeshComponent.PlayAnimation` _arms "/Game/TheAtlant_Content/GA/Bras/Anim/Anim_Reload_Bras_v2.Anim_Reload_Bras_v2" false)
      (bind _harpoonmesh (`self.HarpoonMesh`)
        (:`then`
          (`SkeletalMeshComponent.PlayAnimation` _harpoonmesh "/Game/TheAtlant_Content/GA/Harpon/Animations/harpon_walk.harpon_walk" false)
          (bind _harpoontip (`self.HarpoonTip`)
            (:`then`
              (`SceneComponent.K2_SetRelativeLocation` _harpoontip (-58.0 -136.0 -14.0) false false)
              (`KismetSystemLibrary.Delay` 0.01)
              (`SkeletalMeshComponent.Stop` _harpoonmesh)
              (`SkeletalMeshComponent.Stop` _arms))
            (:`else`)))
        (:`else`)))
    (:`else`)))

(fn `ForceDropDeadBody`
  (params (Item :type "/Game/TheAtlant_Content/BP/BP_ParentItem Object Reference"))
  (returns (Location :type "Vector Structure"))
  (locals (ScaleFactor :type "Float (double-precision)" :default 10.0))
  (bind (_returnvalue_roll _returnvalue_pitch _returnvalue_yaw) (`KismetMathLibrary.BreakRotator` (`self.K2_GetActorRotation`)))
  (if (`/Game/TheAtlant_Content/BP/BP_ParentItem.IsDeadBody` Item)
    (set `local.ScaleFactor` 1.0))
  (bind _collision (`/Game/TheAtlant_Content/BP/BP_ParentItem.Collision` Item)
    (:`then`
      (bind (_returnvalue_x _returnvalue_y _returnvalue_z) (`KismetMathLibrary.BreakVector` (* (`BoxComponent.GetScaledBoxExtent` _collision) (`local.ScaleFactor`))))
      (bind _returnvalue (+ (`self.K2_GetActorLocation`) (`KismetMathLibrary.MakeVector` 0.0 0.0 (+ 0.01 _returnvalue_z))))
      (bind _outhit (`KismetSystemLibrary.BoxTraceSingleForObjects` :`Start` _returnvalue :`End` _returnvalue :`HalfSize` (`KismetMathLibrary.MakeVector` _returnvalue_x _returnvalue_y _returnvalue_z) :`Orientation` (`KismetMathLibrary.MakeRotator` 0.0 0.0 _returnvalue_yaw) :`ObjectTypes` (`|MakeArray` "ObjectTypeQuery1" "ObjectTypeQuery2" "ObjectTypeQuery4" "ObjectTypeQuery6" "ObjectTypeQuery3" "ObjectTypeQuery5" :!type "EObjectTypeQuery Enum") :`DrawDebugType` "Persistent"))
      (return (+ (`.Location` (`GameplayStatics.BreakHitResult` _outhit)) (`self.K2_GetActorLocation`))))
    (:`else`)))

(fn `LookIfShootIntoPlayer`
  (returns (HitPlayer :type Boolean))
  (bind _harpoonspawnpoint (`self.HarpoonSpawnPoint`)
    (:`then`
      (bind _returnvalue (`SceneComponent.K2_GetComponentLocation` _harpoonspawnpoint))
      (bind (_outhit _returnvalue_2) (`KismetSystemLibrary.SphereTraceSingleForObjects` :`Start` _returnvalue :`End` _returnvalue :`Radius` 4.0 :`ObjectTypes` (`|MakeArray` "ObjectTypeQuery7" :!type "EObjectTypeQuery Enum") :`bIgnoreSelf` false))
      (return _returnvalue_2))
    (:`else`)))

(fn `RadioPlayer`
  (params (Clip :type "SoundCue Object Reference"))
  (bind _radio (`self.Radio`))
  (`AudioComponent.Stop` _radio)
  (`AudioComponent.SetSound` _radio Clip)
  (`AudioComponent.Play` _radio 0.0))

(fn `UserConstructionScript`
  ;[1 1 1] Make sure that to store the player transform
  (bind _asgi_the_atlant (cast `/Game/TheAtlant_Content/BP/Game/GI_TheAtlant` (`GameplayStatics.GetGameInstance`)))
  (set `/Game/TheAtlant_Content/BP/Game/GI_TheAtlant.PlayerRespawnTransform` (`self.GetTransform`) _asgi_the_atlant)
  (`KismetSystemLibrary.PrintString` "Setup position" false))