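; BP_SaveSceneManager is a level actor that persists the transforms and alive state of a set of scene objects through GI_TheAtlant.
; On BeginPlay it reads the saved list for its ID, then repositions or destroys each CurrentObjects entry by array index, or builds a fresh list if none exists.
; CE_SaveScene snapshots every object, marking invalid references as dead, and writes the list back to the Game Instance.
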(event `self.ReceiveBeginPlay`
  ;[1 1 1] Get Object list
  (bind _asgi_the_atlant (cast `/Game/TheAtlant_Content/BP/Game/GI_TheAtlant` (`GameplayStatics.GetGameInstance`)))
  (bind _output_get (set `self.SaveObjectList` (`.ObjectList_3_5B121CE8438B2E4E9ECD64A1D55D76AC` (break `/Game/TheAtlant_Content/Data/Struct/S_SaveLevelData` (`|GetArrayItem` (`/Game/TheAtlant_Content/BP/Game/GI_TheAtlant.SaveLevelList` _asgi_the_atlant) (`self.ID`))))))
  ;[1 1 1] Look if has created object list
  (if (!= (`KismetArrayLibrary.Array_Length` _output_get) 0)
    ;[1 1 1] Look if is correct list
    (if (!= (`KismetArrayLibrary.Array_Length` (`self.SaveObjectList`)) (`KismetArrayLibrary.Array_Length` (`self.CurrentObjects`)))
      (`KismetSystemLibrary.PrintString` "Save Object List isn't valid")
      (else
        ;[1 1 1] Load list
        (for (_array_element _array_index) (`self.CurrentObjects`)
          (bind (_index _transform _isalive) (break `/Game/TheAtlant_Content/Data/Struct/S_SaveObjectData` (`|GetArrayItem` (`self.SaveObjectList`) _array_index)))
          (if (== _array_index _index)
            (if _isalive
              (`self.K2_SetActorTransform` _array_element _transform false false)
              (else
                (`self.K2_DestroyActor` _array_element)))
            (else
              (`KismetSystemLibrary.PrintString` "Object isn't valid"))))))
    (else
      ;[1 1 1] Create list
      (for (_array_element_2 _array_index_2) (`self.CurrentObjects`)
        (`self.CreateNewSaveObjectDataEntry` _array_index_2 _array_element_2))
      (`KismetSystemLibrary.PrintString` "Create List"))))

(event `CE_SaveScene`
  (bind _tempsaveobjectlist (`self.TempSaveObjectList`))
  ;[1 1 1] Save object on scene
  (`KismetArrayLibrary.Array_Clear` (`self.TempSaveObjectList`))
  (for (_array_element _array_index) (`self.CurrentObjects`)
    (if (`KismetSystemLibrary.IsValid` _array_element)
      (`KismetArrayLibrary.Array_Add` (`self.TempSaveObjectList`) (make `/Game/TheAtlant_Content/Data/Struct/S_SaveObjectData` _array_index (`self.GetTransform` _array_element) true))
      (else
        (`KismetArrayLibrary.Array_Add` (`self.TempSaveObjectList`) (make `/Game/TheAtlant_Content/Data/Struct/S_SaveObjectData` _array_index (`KismetMathLibrary.MakeTransform` (0.0 0.0 0.0)))))))
  ;[1 1 1] Save Temp list to Game Instance
  (set `self.SaveObjectList` _tempsaveobjectlist)
  (bind _asgi_the_atlant (cast `/Game/TheAtlant_Content/BP/Game/GI_TheAtlant` (`GameplayStatics.GetGameInstance`)))
  (`KismetArrayLibrary.Array_Set` (`/Game/TheAtlant_Content/BP/Game/GI_TheAtlant.SaveLevelList` _asgi_the_atlant) (`self.ID`) (make `/Game/TheAtlant_Content/Data/Struct/S_SaveLevelData` _tempsaveobjectlist) true))

(fn `CreateNewSaveObjectDataEntry`
  (params (Index :type Integer) (Actor :type "Actor Object Reference"))
  (`KismetArrayLibrary.Array_Add` (`self.SaveObjectList`) (make `/Game/TheAtlant_Content/Data/Struct/S_SaveObjectData` Index (`self.GetTransform` Actor) true)))

(fn `UserConstructionScript`)