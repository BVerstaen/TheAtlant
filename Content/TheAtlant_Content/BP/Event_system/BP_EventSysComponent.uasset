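; BP_EventSysComponent is a reusable sphere trigger that fires an event on its parent actor through BPI_EventFunctions.
; Construction sizes the hitbox and caches the parent actor, or disables collision when the radius is near zero.
; Beginning overlap calls the parent's event and disables the trigger; ending overlap re-enables it unless one-shot.
; Tick draws a debug sphere colored by enabled state, and overlaps do not filter the overlapping actor.
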(event `self.Sphere_Hitbox.OnComponentBeginOverlap`
  (params (OverlappedComponent :type "PrimitiveComponent Object Reference") (OtherActor :type "Actor Object Reference") (OtherComp :type "PrimitiveComponent Object Reference") (OtherBodyIndex :type Integer) (bFromSweep :type Boolean) (SweepResult :type "HitResult Structure (by ref)"))
  ;[0.3144 0.2917 1] Check and call event
  (if (`self._PlayerInsideEventRadius`)
    (`KismetSystemLibrary.PrintString` "Event is disabled" :!label _label)
    (elif (`self._isEnabled`)
      (if (`KismetSystemLibrary.DoesImplementInterface` (`self._Parent`) "/Game/TheAtlant_Content/BP/Event_system/BPI_EventFunctions.BPI_EventFunctions_C")
        (set `self._isEnabled` false)
        (set `self._PlayerInsideEventRadius` true)
        (message `/Game/TheAtlant_Content/BP/Event_system/BPI_EventFunctions.CallEvent` (`self._Parent`))
        (`KismetSystemLibrary.PrintString` "Event is playing and now disabled")
        (else
          (`KismetSystemLibrary.PrintString` "No event system")))
      (else
        (goto _label)))))

(event `self.Sphere_Hitbox.OnComponentEndOverlap`
  (params (OverlappedComponent :type "PrimitiveComponent Object Reference") (OtherActor :type "Actor Object Reference") (OtherComp :type "PrimitiveComponent Object Reference") (OtherBodyIndex :type Integer))
  ;[1 0.1938 0.4226] Re-enable event if repeatable
  (set `self._PlayerInsideEventRadius` false)
  (if (`self._isOneShot`)
    (`KismetSystemLibrary.PrintString` "Event was one shot and wont be reenabled")
    (else
      (set `self._isEnabled` true)
      (`KismetSystemLibrary.PrintString` "Player is outside the radius  and event is now enabled"))))

(event `self.ReceiveTick`
  (params (DeltaSeconds :type "Float (single-precision)"))
  (bind _sphere_hitbox (`self.Sphere_Hitbox`))
  ;[1 1 1] Visualize Hitbox in debug mode (for designers)
  (`KismetSystemLibrary.DrawDebugSphere` (`SceneComponent.K2_GetComponentLocation` _sphere_hitbox) (`SphereComponent.SphereRadius` _sphere_hitbox) 12 (`KismetMathLibrary.SelectColor` (struct :`R` 1.0 :`G` 1.0 :`B` 1.0 :`A` 1.0) (struct :`R` 1.0 :`G` 0.097019 :`A` 1.0) (`self._isEnabled`))))

(fn `UserConstructionScript`
  (bind __hitboxtriggerradius (`self._hitboxTriggerRadius`))
  (bind _sphere_hitbox (`self.Sphere_Hitbox`))
  ;[1 1 1] Hitbox Handling
  (if (>= __hitboxtriggerradius 0.1)
    (`SphereComponent.SetSphereRadius` _sphere_hitbox __hitboxtriggerradius true)
    (set `self._Parent` (`self.GetParentActor`))
    (else
      (`PrimitiveComponent.SetCollisionEnabled` _sphere_hitbox "NoCollision"))))