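; BP_EventCrashGame is a trigger-box event object that quits the game when overlapped, with no check on which actor enters.
; Begin overlap checks the enabled and inside-radius flags, disables the event, then runs CallEvent, which calls QuitGame rather than causing an actual crash.
; End overlap clears the inside flag and re-enables the event unless it is one-shot.
; Debug prints report state; the box-drawing code is disconnected.
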(event `self.Box.OnComponentBeginOverlap`
  (params (OverlappedComponent :type "PrimitiveComponent Object Reference") (OtherActor :type "Actor Object Reference") (OtherComp :type "PrimitiveComponent Object Reference") (OtherBodyIndex :type Integer) (bFromSweep :type Boolean) (SweepResult :type "HitResult Structure (by ref)"))
  ;[0.3144 0.2917 1] Check and call event
  (if (`self._PlayerInsideEventRadius`)
    (`KismetSystemLibrary.PrintString` "Event is disabled" :!label _label)
    (elif (`self._isEnabled`)
      (set `self._isEnabled` false)
      (set `self._PlayerInsideEventRadius` true)
      (`/Game/TheAtlant_Content/BP/Event_system/BPI_EventFunctions.CallEvent`)
      (`KismetSystemLibrary.PrintString` "Event is playing and now disabled")
      (else
        (goto _label)))))

(event `self.Box.OnComponentEndOverlap`
  (params (OverlappedComponent :type "PrimitiveComponent Object Reference") (OtherActor :type "Actor Object Reference") (OtherComp :type "PrimitiveComponent Object Reference") (OtherBodyIndex :type Integer))
  ;[1 0.1938 0.4226] Re-enable event if repeatable
  (set `self._PlayerInsideEventRadius` false)
  (if (`self.Is One Shot`)
    (`KismetSystemLibrary.PrintString` "Event was one shot and wont be reenabled")
    (else
      (set `self._isEnabled` true)
      (`KismetSystemLibrary.PrintString` "Player is outside the radius  and event is now enabled"))))

(event `self.ReceiveTick`
  (params (DeltaSeconds :type "Float (single-precision)"))
  ;[1 1 1] Draw
)

(event `self.CallEvent`
  (`KismetSystemLibrary.QuitGame` null "Quit"))

(fn `UserConstructionScript`)