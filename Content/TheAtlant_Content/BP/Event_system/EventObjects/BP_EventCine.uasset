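; BP_EventCine is an event object that plays a level sequence cinematic when CallEvent fires, optionally only once.
; It plays an optional 2D sound, then sets the assigned cine camera's focus to smoothly track the player pawn and starts the sequencer.
; With no valid camera it only prints a warning, and the camera shake helper is unconnected and does nothing.
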(event `self.CallEvent`
  (bind _cameracomponent (`self.CameraComponent`))
  (if (`self.PlayOnce`)
    (if (not (`self.used`))
      (set `self.used` true)
      (`self.PlaySoundIfAny` :!label _label)
      (if (`KismetSystemLibrary.IsValid` _cameracomponent)
        (set `CineCameraComponent.FocusSettings` (make `CameraFocusSettings` "Tracking" 100000.0 (make `CameraTrackingFocusSettings` (`|ConvertAsset` (`GameplayStatics.GetPlayerPawn` 0))) true) (`CineCameraActor.GetCineCameraComponent` _cameracomponent))
        (`MovieSceneSequencePlayer.Play` (`LevelSequenceActor.SequencePlayer` (`self.LevelSequencer`)))
        (else
          (`KismetSystemLibrary.PrintString` "No camera set"))))
    (else
      (goto _label))))

(fn `PlayCamShakeIfAny`)

(fn `PlaySoundIfAny`
  (bind _sound (`self.Sound`))
  (if (`KismetSystemLibrary.IsValid` _sound)
    (`GameplayStatics.SpawnSound2D` _sound 1.0 1.0 0.0 null)))

(fn `UserConstructionScript`)