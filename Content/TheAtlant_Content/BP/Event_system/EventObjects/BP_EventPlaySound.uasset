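; BP_EventPlaySound is an event-system object that plays a sound at its own location when CallEvent fires.
; CallEvent checks a Used flag, spawns SoundObjectRef at the root's position and binds to its audio-finished callback.
; In one-time mode the actor destroys itself when playback ends, though the Used assignment only writes back its own value.
; NoSoundSet is an empty stub.
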(event `self.CallEvent`
  (if (not (`self.Used`))
    (if (`self.IsOneTimeUse`)
      (set `self.Used` (`self.Used`)))
    (bind _returnvalue (`GameplayStatics.SpawnSoundAtLocation` (`self.SoundObjectRef`) (`SceneComponent.K2_GetComponentLocation` (`self.DefaultSceneRoot`)) (struct) 1.0 1.0 0.0 null null))
    (add `AudioComponent.OnAudioFinished` _returnvalue (delegate `OnAudioFinished_Event`))))

(event `OnAudioFinished_Event`
  (if (`self.IsOneTimeUse`)
    (`self.K2_DestroyActor`)))

(fn `NoSoundSet`)

(fn `UserConstructionScript`)