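; An event object in the event system that plays a referenced sound at a separate location when triggered.
; CallEvent spawns the sound at the world position of its SoundPosition component and binds to the audio-finished delegate.
; When playback ends, the actor destroys itself if flagged as one-time use.
; Tick draws a debug sphere to show the sound location, while the construction script and NoSoundSet function are empty.
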(event `self.CallEvent`
  (bind _returnvalue (`GameplayStatics.SpawnSoundAtLocation` (`self.SoundObjectRef`) (`SceneComponent.K2_GetComponentLocation` (`self.SoundPosition`)) (struct) 1.0 1.0 0.0 null null))
  (add `AudioComponent.OnAudioFinished` _returnvalue (delegate `OnAudioFinished_Event`)))

(event `OnAudioFinished_Event`
  (if (`self.IsOneTimeUse`)
    (`self.K2_DestroyActor`)))

(event `self.ReceiveTick`
  (params (DeltaSeconds :type "Float (single-precision)"))
  ;[1 1 1] Visualize  Sound Location
  (`KismetSystemLibrary.DrawDebugSphere` (`SceneComponent.K2_GetComponentLocation` (`self.SoundPosition`)) 30.0))

(fn `NoSoundSet`)

(fn `UserConstructionScript`)