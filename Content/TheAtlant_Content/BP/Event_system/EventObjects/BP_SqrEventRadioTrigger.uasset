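; Box-volume event trigger that plays a radio transmission, with HUD text and sound, when something overlaps it.
; Overlap calls the event and disables it until overlap ends, with separate one-shot and one-time-use flags limiting repeats.
; ShowRadioText steps through the script array by re-calling itself after each delay, while BP_Player's RadioPlayer handles the sound.
; Tick optionally draws the box for debugging.
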(event `Called`
  (if (`self.IsOneTimeUse`)
    (if (not (`self.Used`))
      (set `self.Used` true)
      (`KismetSystemLibrary.PrintString` "Bruh" :!label _label)
      (if (> (`KismetArrayLibrary.Array_Length` (`self.RadioScript`)) 0)
        (`KismetSystemLibrary.PrintString` "Bruh2")
        (`self.ShowRadioText`)
        (`self.PlayRadioSound`)
        (else
          (`self.PlayRadioSound`))))
    (else
      (goto _label))))

(event `ShowRadioText`
  ;[1 1 1] Radio Text
  (bind _ashud_the_atlant (cast `/Game/TheAtlant_Content/BP/Game/HUD_TheAtlant` (`PlayerController.GetHUD` (`GameplayStatics.GetPlayerController` 0)))
    (:`then`
      ;;[1 1 1] For each loop inside script array
      (`/Game/TheAtlant_Content/BP/Game/HUD_TheAtlant.CE_DisplayMessage` _ashud_the_atlant (`|GetArrayItem` (`self.RadioScript`) (`self.arrayIndex`)) (`self.RadioColor`) (`self.RadioDuration`))
      (`/Engine/EditorBlueprintResources/StandardMacros.IncrementInt` (`self.arrayIndex`)
        (:`  `
          (if (< (`self.arrayIndex`) (`KismetArrayLibrary.Array_Length` (`self.RadioScript`)))
            (`KismetSystemLibrary.Delay` (`self.RadioDuration`))
            (`self.ShowRadioText`)
            (else
              (set `self.arrayIndex` 0))))))
    (:`CastFailed`
      (`KismetSystemLibrary.PrintString` "error"))))

(event `self.ReceiveTick`
  (params (DeltaSeconds :type "Float (single-precision)"))
  (bind _box (`self.Box`))
  ;[1 1 1] Draw
  (if (`self.DrawBox`)
    (`KismetSystemLibrary.DrawDebugBox` (`SceneComponent.K2_GetComponentLocation` _box) (`BoxComponent.GetScaledBoxExtent` _box) (struct :`G` 1.0 :`B` 0.150077 :`A` 1.0) (`SceneComponent.K2_GetComponentRotation` _box) 0.4 1.0)))

(event `PlayRadioSound`
  ;[1 1 1] Play sound
  (bind _asbp_player (cast `/Game/TheAtlant_Content/BP/BP_Player` (`GameplayStatics.GetPlayerPawn` 0)))
  (`/Game/TheAtlant_Content/BP/BP_Player.RadioPlayer` _asbp_player (`self.SoundObjectRef`)))

(event `self.Box.OnComponentBeginOverlap`
  (params (OverlappedComponent :type "PrimitiveComponent Object Reference") (OtherActor :type "Actor Object Reference") (OtherComp :type "PrimitiveComponent Object Reference") (OtherBodyIndex :type Integer) (bFromSweep :type Boolean) (SweepResult :type "HitResult Structure (by ref)"))
  ;[0.3144 0.2917 1] Check and call event
  (if (`self._PlayerInsideEventRadius`)
    (`KismetSystemLibrary.PrintString` "Event is disabled" :!label _label_2)
    (elif (`self._isEnabled`)
      (set `self._isEnabled` false)
      (set `self._PlayerInsideEventRadius` true)
      (`self.Called`)
      (`KismetSystemLibrary.PrintString` "Event is playing and now disabled")
      (else
        (goto _label_2)))))

(event `self.Box.OnComponentEndOverlap`
  (params (OverlappedComponent :type "PrimitiveComponent Object Reference") (OtherActor :type "Actor Object Reference") (OtherComp :type "PrimitiveComponent Object Reference") (OtherBodyIndex :type Integer))
  ;[1 0.1938 0.4226] Re-enable event if repeatable
  (set `self._PlayerInsideEventRadius` false)
  (if (`self.Is One Shot`)
    (`KismetSystemLibrary.PrintString` "Event was one shot and wont be reenabled")
    (else
      (set `self._isEnabled` true)
      (`KismetSystemLibrary.PrintString` "Player is outside the radius  and event is now enabled"))))

(fn `UserConstructionScript`)